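; Player Blueprint that creates the WBP_Inventaire widget and drives its inventory by index, without mouse input.
; E opens the inventory or selects the highlighted item; B deselects or closes it.
; Directional events step through a flattened five-wide grid, or through the option buttons once an item is selected, recoloring the focus.
; Selection widens a grid column to reveal that item's option box, found at a 15-child offset from its image.
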(event `self.ReceiveBeginPlay`
  (`parent.ReceiveBeginPlay`)
  (bind _returnvalue (`|CreateWidget` "/Game/PrototypeGame/Inventaire/WBP_Inventaire.WBP_Inventaire_C"))
  (set `self.WBP_Inventaire` _returnvalue)
  (set `self.X_MaxInventory` 4)
  (set `self.Y_MaxInventory` 10)
  (set `self.CurrentIndex` 0)
  (set `self.Z_MaxIndexItemOption` 3)
  (set `self.ColumnIndex` 1)
  (set `self.ColumnMaxIndex` 9))

(event `Key|E`
  (params (Key :type "Key Structure"))
  (bind _wbp_inventaire (`self.WBP_Inventaire`))
  (:`Pressed`
    (if (`Widget.IsInViewport` _wbp_inventaire)
      (`self.SelectionInventory` (`self.IsSelected`))
      (else
        (`self.NavigationInventory`)
        (`UserWidget.AddToViewport` _wbp_inventaire 0)))))

(event `Key|B`
  (params (Key :type "Key Structure"))
  (bind _wbp_inventaire (`self.WBP_Inventaire`))
  (:`Pressed`
    (if (`Widget.IsInViewport` _wbp_inventaire)
      (if (`self.IsSelected`)
        (`self.UnSelectInventory`)
        (else
          (`Widget.RemoveFromParent` _wbp_inventaire))))))

(event `DRightInnventory`
  ;[0 0.774 1] Déplacement clavier Inventaire par index
  (if (not (`self.IsSelected`))
    (bind _isless (`self.Maxi` (`self.X_IndexInventory`) (`self.X_MaxInventory`)))
    (if _isless
      (set `self.X_IndexInventory` (+ (`self.X_IndexInventory`) 1))
      (bind _isless_2 (`self.Maxi` (`self.ColumnIndex`) (`self.ColumnMaxIndex`)))
      (if _isless_2
        (set `self.ColumnIndex` (+ 2 (`self.ColumnIndex`)))
        (if (`Widget.IsInViewport` (`self.WBP_Inventaire`)) :!label _label
          (`self.NavigationInventory`))))))

(event `DLeftInventory`
  ;[0 0.774 1] Déplacement clavier Inventaire par index
  (if (not (`self.IsSelected`))
    (bind _isgreater (`self.Minimum` (`self.X_IndexInventory`)))
    (if _isgreater
      (set `self.X_IndexInventory` (- (`self.X_IndexInventory`) 1))
      (bind _isgreater_2 (`self.Minimum` (`self.ColumnIndex`) 1))
      (if _isgreater_2
        (set `self.ColumnIndex` (- (`self.ColumnIndex`) 2))
        (goto _label)))))

(event `DDownInventory`
  (bind _z_indexitemoption (`self.Z_IndexItemOption`))
  ;[0 0.774 1] Déplacement clavier Inventaire par index
  (if (`self.IsSelected`)
    (bind _isless (`self.Maxi` _z_indexitemoption (`self.Z_MaxIndexItemOption`)))
    (if _isless
      (`self.NavigationInfoIntem` (+ _z_indexitemoption 1) _z_indexitemoption))
    (else
      (bind _isless_2 (`self.Maxi` (`self.Y_IndexInventory`) (`self.Y_MaxInventory`)))
      (if _isless_2
        (set `self.Y_IndexInventory` (+ (`self.Y_IndexInventory`) 5))
        (goto _label)))))

(event `DUpInventory`
  (bind _z_indexitemoption (`self.Z_IndexItemOption`))
  ;[0 0.774 1] Déplacement clavier Inventaire par index
  (if (`self.IsSelected`)
    (bind _isgreater (`self.Minimum` _z_indexitemoption))
    (if _isgreater
      (`self.NavigationInfoIntem` (- _z_indexitemoption 1) _z_indexitemoption))
    (else
      (bind _isgreater_2 (`self.Minimum` (`self.Y_IndexInventory`)))
      (if _isgreater_2
        (set `self.Y_IndexInventory` (- (`self.Y_IndexInventory`) 5))
        (goto _label)))))

(fn `Maxi`
  (params (Value :type Integer) (Max :type Integer))
  (returns (IsLess :type Boolean))
  (return (> Max Value)))

(fn `Minimum`
  (params (Value :type Integer) (Minimum :type Integer))
  (returns (IsGreater :type Boolean))
  (return (> Value Minimum)))

(fn `NavigationInfoIntem`
  (params (NewIndex :type Integer) (CurrentIndex :type Integer))
  (bind _returnvalue (`PanelWidget.GetChildAt` (`/Game/PrototypeGame/Inventaire/WBP_Inventaire.Inventory` (`self.WBP_Inventaire`)) (+ (`self.CurrentIndex`) 15)))
  (bind _asvertical_box (cast `VerticalBox` _returnvalue))
  (bind _asbutton (cast `Button` (`PanelWidget.GetChildAt` _asvertical_box CurrentIndex)))
  (`Button.SetBackgroundColor` _asbutton (struct :`R` 1.0 :`G` 1.0 :`B` 1.0 :`A` 1.0))
  (bind _asvertical_box_2 (cast `VerticalBox` _returnvalue))
  (bind _asbutton_2 (cast `Button` (`PanelWidget.GetChildAt` _asvertical_box_2 NewIndex)))
  (`Button.SetBackgroundColor` _asbutton_2 (struct :`R` 1.0 :`B` 1.0 :`A` 1.0))
  (set `self.Z_IndexItemOption` NewIndex))

(fn `NavigationInventory`
  (bind _returnvalue (+ (`self.Y_IndexInventory`) (`self.X_IndexInventory`)))
  (bind _asimage (cast `Image` (`PanelWidget.GetChildAt` (`/Game/PrototypeGame/Inventaire/WBP_Inventaire.Inventory` (`self.WBP_Inventaire`)) (`self.CurrentIndex`)))
    (:`then`
      (`Image.SetColorAndOpacity` _asimage (struct :`R` 1.0 :`G` 1.0 :`B` 1.0 :`A` 1.0))
      (bind _asimage_2 (cast `Image` (`PanelWidget.GetChildAt` (`/Game/PrototypeGame/Inventaire/WBP_Inventaire.Inventory` (`self.WBP_Inventaire`)) _returnvalue))
        (:`then`
          (`Image.SetColorAndOpacity` _asimage_2 (struct :`R` 1.0 :`B` 1.0 :`A` 1.0))
          (set `self.CurrentIndex` _returnvalue))
        (:`CastFailed`
          (`KismetSystemLibrary.PrintString` "FAILED CAST " true true (struct :`R` 1.0 :`A` 1.0)))))
    (:`CastFailed`
      (`KismetSystemLibrary.PrintString` "FAILED CAST " true true (struct :`R` 1.0 :`A` 1.0)))))

(fn `SelectionInventory`
  (params (IsSelected :type Boolean))
  (bind _inventory (`/Game/PrototypeGame/Inventaire/WBP_Inventaire.Inventory` (`self.WBP_Inventaire`)))
  (if (not IsSelected)
    (bind _asimage (cast `Image` (`PanelWidget.GetChildAt` (`/Game/PrototypeGame/Inventaire/WBP_Inventaire.Inventory` (`self.WBP_Inventaire`)) (`self.CurrentIndex`))))
    (set `Image.ColorAndOpacity` (struct :`R` 1.0 :`A` 1.0) _asimage)
    (set `self.IsSelected` true)
    (`GridPanel.SetColumnFill` _inventory (`self.ColumnIndex`) 2.0)
    (bind _asvertical_box (cast `VerticalBox` (`PanelWidget.GetChildAt` _inventory (+ 15 (`self.CurrentIndex`)))))
    (`Widget.SetVisibility` _asvertical_box "Visible")
    (bind _asbutton (cast `Button` (`PanelWidget.GetChildAt` _asvertical_box 0)))
    (`Button.SetBackgroundColor` _asbutton (struct :`R` 1.0 :`B` 1.0 :`A` 1.0))))

(fn `UnSelectInventory`
  (bind _inventory (`/Game/PrototypeGame/Inventaire/WBP_Inventaire.Inventory` (`self.WBP_Inventaire`)))
  (if true
    (bind _asimage (cast `Image` (`PanelWidget.GetChildAt` (`/Game/PrototypeGame/Inventaire/WBP_Inventaire.Inventory` (`self.WBP_Inventaire`)) (`self.CurrentIndex`))))
    (set `Image.ColorAndOpacity` (struct :`R` 1.0 :`B` 1.0 :`A` 1.0) _asimage)
    (set `self.IsSelected` true)
    (`GridPanel.SetColumnFill` _inventory (`self.ColumnIndex`) 0.1)
    (bind _asvertical_box (cast `VerticalBox` (`PanelWidget.GetChildAt` _inventory (+ 15 (`self.CurrentIndex`)))))
    (`Widget.SetVisibility` _asvertical_box "Collapsed")
    (bind _asbutton (cast `Button` (`PanelWidget.GetChildAt` _asvertical_box (`self.Z_IndexItemOption`))))
    (`Button.SetBackgroundColor` _asbutton (struct :`R` 1.0 :`G` 1.0 :`B` 1.0 :`A` 1.0))
    (set `self.IsSelected` false)
    (set `self.Z_IndexItemOption` 0)))

(fn `UserConstructionScript`
  (`parent.UserConstructionScript`))