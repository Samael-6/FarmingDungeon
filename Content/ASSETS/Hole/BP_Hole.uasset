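; BP_Hole is a planting hole that grows a received item into a crop.
; Activation of BPC_CanReceiveItem plants the item if the hole is unoccupied, ends the player's hold, and looks up growth data in DT_Crops.
; A self-calling one-second Delay counts toward each phase's duration, revealing the filled hole and sprout meshes.
; On reaching Finished, it spawns the crop actor and destroys itself.
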(event `self.BPC_CanReceiveItem.OnComponentActivated`
  (params (Component :type "ActorComponent Object Reference") (bReset :type Boolean))
  (if (`|EnumEquality` (`self.ItemContained`) "NewEnumerator15")
    (`self.PutItemIntoHole` (`/Game/FarmingDungeon/Blueprints/Components/BPC_CanReceiveItem.receivingItem` (`self.BPC_CanReceiveItem`)))
    (bind _returnvalue (`GameplayStatics.GetActorOfClass` "/Game/FarmingDungeon/Blueprints/Characters/BP_Player.BP_Player_C"))
    (`/Game/FarmingDungeon/Blueprints/Characters/BP_Player.StopHoldAnimation` _returnvalue)
    (`/Game/FarmingDungeon/Blueprints/Characters/BP_Player.StopHolding` _returnvalue true)))

(event `Timer`
  (`KismetSystemLibrary.Delay` 1.0)
  (bind _output_get (set `self.CurrentTime` (+ (`self.CurrentTime`) 1)))
  (if (>= _output_get (`self.NextStateTime`))
    (bind _continue_ (`self.GoToNextPhase`))
    (if _continue_
      (`self.Timer`))
    (else
      (`self.Timer`))))

(fn `GetBreakFromCrop`
  (params (Item :type "/Game/FarmingDungeon/Blueprints/Manager/E_Items Enum" :default "NewEnumerator15"))
  (returns (ReturnValue :type "/Game/FarmingDungeon/Blueprints/Manager/DataTables/Field/ST_Crops Structure"))
  (locals (NewLocalVar :type Name :default "None") (tempRowNmae :type Name))
  (bind _outrownames (`DataTableFunctionLibrary.GetDataTableRowNames` "/Game/FarmingDungeon/Blueprints/Manager/DataTables/Field/DT_Crops.DT_Crops"))
  (for _array_element _outrownames
    (bind _returnvalue (`|GetDataTableRow` "/Game/FarmingDungeon/Blueprints/Manager/DataTables/Field/DT_Crops.DT_Crops" _array_element)
      (:`then`
        (if (`|EnumEquality` (`.Item_2_CE94BCEF478799541F9208B9A0158347` (break `/Game/FarmingDungeon/Blueprints/Manager/DataTables/Field/ST_Crops` _returnvalue)) Item)
          (set `local.tempRowNmae` _array_element)
          (break)))
      (:`RowNotFound`
        (return (stale _returnvalue_2)))))
  (bind _returnvalue_2 (`|GetDataTableRow` "/Game/FarmingDungeon/Blueprints/Manager/DataTables/Field/DT_Crops.DT_Crops" (`local.tempRowNmae`))
    (:`then`
      (return _returnvalue_2))))

(fn `GoToNextPhase`
  (returns (`Continue?` :type Boolean))
  (bind _nextstate (`self.NextState`))
  (if (`|EnumEquality` _nextstate "NewEnumerator2")
    (`|SpawnActorFromClass` (`.Bp_Crops_10_272C3EBA48B387936C063F96C8E6F902` (break `/Game/FarmingDungeon/Blueprints/Manager/DataTables/Field/ST_Crops` (`self.GetBreakFromCrop` (`self.ItemContained`)))) (`KismetMathLibrary.MakeTransform` (`self.K2_GetActorLocation`)) "Undefined" "MultiplyWithRoot" null null)
    (`self.K2_DestroyActor`)
    (else
      (set `self.CurrentState` _nextstate)
      (`self.SetPhaseInfo`)
      (set `self.CurrentTime` 0)
      (return true))))

(fn `PutItemIntoHole`
  (params (Item :type "/Game/FarmingDungeon/Blueprints/Manager/E_Items Enum" :default "NewEnumerator15"))
  (locals (tempRowNmae :type Name))
  (set `self.ItemContained` Item)
  (set `self.GrowPhase` (`.MemberVar_3_6_9BF678104F0E6B15237D04B8684EAB40` (break `/Game/FarmingDungeon/Blueprints/Manager/DataTables/Field/ST_Crops` (`self.GetBreakFromCrop` Item))))
  (set `self.CurrentTime` 0)
  (set `self.CurrentState` "NewEnumerator0")
  (`self.SetPhaseInfo`)
  (`self.Timer`))

(fn `SetPhaseInfo`
  (bind _growphase (`self.GrowPhase`))
  (bind _currentstate (`self.CurrentState`))
  (bind _keys (`BlueprintMapLibrary.Map_Keys` _growphase))
  (bind _values (`BlueprintMapLibrary.Map_Values` _growphase))
  (set `self.NextStateTime` (`|GetArrayItem` _values (`KismetArrayLibrary.Array_Find` _keys _currentstate)))
  (switch `/Game/FarmingDungeon/Blueprints/Manager/E_GrowState` _currentstate
    (:`NewEnumerator0`
      (set `self.NextState` "NewEnumerator1")
      (`SceneComponent.SetHiddenInGame` (`self.FullHole`) false false :!label _label))
    (:`NewEnumerator1`
      (set `self.NextState` "NewEnumerator2")
      (`SceneComponent.SetHiddenInGame` (`self.Sprout`) false false)
      (goto _label))
    (:`NewEnumerator2`
      (set `self.NextState` "NewEnumerator3"))))

(fn `UserConstructionScript`)