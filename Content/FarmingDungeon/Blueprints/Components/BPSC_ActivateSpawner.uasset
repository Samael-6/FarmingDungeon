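; Component that sets up monster and resource spawners for the current dungeon in the farming dungeon game.
; CheckDungeon finds the first true IsLevel flag in the game instance and loads the F or M dungeon's monster list, resource list and level.
; With over three monster spawners, ActivationSpawnerMonster randomly switches some off, then feeds that data to active ones and spawns.
; ActivationSpawnerRessource passes the resource list to every resource spawner.
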(event `self.ReceiveBeginPlay`
  (bind _asbp_game_instance (cast `/Game/FarmingDungeon/Blueprints/Manager/BP_GameInstance` (`GameplayStatics.GetGameInstance`)))
  (set `self.BP_GameInstance_Ref` _asbp_game_instance)
  (bind _outactors (`GameplayStatics.GetAllActorsOfClass` "/Game/FarmingDungeon/Blueprints/Actors/BP_Monstres/BP_SpawnerMonstre.BP_SpawnerMonstre_C"))
  (set `self.ListeSpawner` _outactors))

(fn `ActivationSpawnerMonster`
  (bind _outactors (`GameplayStatics.GetAllActorsOfClass` "/Game/FarmingDungeon/Blueprints/Actors/BP_Monstres/BP_SpawnerMonstre.BP_SpawnerMonstre_C"))
  (bind _returnvalue (`KismetArrayLibrary.Array_Length` _outactors))
  (if (> _returnvalue 3)
    (set `self.NbSpawnerDesactivate` (`KismetMathLibrary.RandomIntegerInRange` 0 (- _returnvalue 3)))
    (while (>= (`self.NbSpawnerDesactivate`) 0)
      (set `/Game/FarmingDungeon/Blueprints/Actors/BP_Monstres/BP_SpawnerMonstre.IsActive` false (`|GetArrayItem` _outactors (`KismetMathLibrary.RandomIntegerInRange` 0 (- _returnvalue 1))))
      (set `self.NbSpawnerDesactivate` (- (`self.NbSpawnerDesactivate`) 1))))
  (for _array_element (`self.ListeSpawner`)
    (if (`/Game/FarmingDungeon/Blueprints/Actors/BP_Monstres/BP_SpawnerMonstre.IsActive` _array_element)
      (`self.CheckDungeon`)
      (`/Game/FarmingDungeon/Blueprints/Actors/BP_Monstres/BP_SpawnerMonstre.MonsterChoice` _array_element (`self.ListeMonstres`) (`self.LvlDungeon`))
      (`/Game/FarmingDungeon/Blueprints/Actors/BP_Monstres/BP_SpawnerMonstre.MonsterChoice` _array_element (`self.ListeMonstres`) (`self.LvlDungeon`))
      (`/Game/FarmingDungeon/Blueprints/Actors/BP_Monstres/BP_SpawnerMonstre.SpawnMonster` _array_element)
      (`KismetSystemLibrary.PrintString` "Hello"))))

(fn `ActivationSpawnerRessource`
  (bind _outactors (`GameplayStatics.GetAllActorsOfClass` "/Game/FarmingDungeon/Blueprints/Actors/BP_Ressources/BP_SpawnerRessources.BP_SpawnerRessources_C"))
  (`self.CheckDungeon`)
  (for _array_element _outactors
    (`/Game/FarmingDungeon/Blueprints/Actors/BP_Ressources/BP_SpawnerRessources.RessourceChoice` _array_element (`self.ListeRessources`))))

(fn `CheckDungeon`
  (bind _bp_gameinstance_ref (`self.BP_GameInstance_Ref`))
  (bind _bp_gameinstance_ref_2 (`self.BP_GameInstance_Ref`))
  (for (_array_element _array_index) (`/Game/FarmingDungeon/Blueprints/Manager/BP_GameInstance.IsLevel` (`self.BP_GameInstance_Ref`))
    (if _array_element
      (break)))
  (switch `int` _array_index
    (:`1`
      (set `self.ListeMonstres` (`/Game/FarmingDungeon/Blueprints/Manager/BP_GameInstance.ListeMonstresF` _bp_gameinstance_ref_2))
      (set `self.LvlDungeon` (`/Game/FarmingDungeon/Blueprints/Manager/BP_GameInstance.Lvl_DungeounF` _bp_gameinstance_ref_2))
      (set `self.ListeRessources` (`/Game/FarmingDungeon/Blueprints/Manager/BP_GameInstance.ListeRessourcesF` (`self.BP_GameInstance_Ref`))))
    (:`2`
      (set `self.ListeMonstres` (`/Game/FarmingDungeon/Blueprints/Manager/BP_GameInstance.ListeMonstresM` _bp_gameinstance_ref))
      (set `self.LvlDungeon` (`/Game/FarmingDungeon/Blueprints/Manager/BP_GameInstance.Lvl_DungeunM` _bp_gameinstance_ref))
      (set `self.ListeRessources` (`/Game/FarmingDungeon/Blueprints/Manager/BP_GameInstance.ListeRessourcesM` (`self.BP_GameInstance_Ref`))))))