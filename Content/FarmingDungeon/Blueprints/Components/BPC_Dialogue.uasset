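; Dialogue component for villagers that steps through a DataTable of numbered rows, supplying speaker, text and player choices.
; Each advance follows the next-row index from the current row or selected choice.
; A set villager condition redirects the row index to the conditional branch and is cleared in CheckVillagerState, which also runs on every row fetch.
; Finishing dialogue can trigger villager movement and calls Isabelle's tutorial hook.
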(event `self.ReceiveTick`
  (params (DeltaSeconds :type "Float (single-precision)")))

(fn `CheckTriggerMovement`
  (if (`.TriggerMovement_36_82F0B2234D260EB161B2CAAE09E4FE6D` (break `/Game/FarmingDungeon/Blueprints/Manager/ST_DialogueRowDatas` (`self.CurrentDialogueRow`)))
    (`/Game/FarmingDungeon/Blueprints/Characters/Villageois/BP_VillagerParent.TriggerMovement` (`self.VillagerParentRef`))))

(fn `CheckVillagerState`
  (returns (VillagerCondition :type Boolean))
  (bind _villagercondition (`/Game/FarmingDungeon/Blueprints/Characters/Villageois/BP_VillagerParent.VillagerCondition` (`self.VillagerParentRef`)))
  (if _villagercondition
    (set `self.CurrentRowNumber` (`.NextRowByCondition_24_4E3BC43C476CEED0D19D07AC061603EF` (break `/Game/FarmingDungeon/Blueprints/Manager/ST_DialogueRowDatas` (`self.CurrentDialogueRow`))))
    (`/Game/FarmingDungeon/Blueprints/Characters/Villageois/BP_VillagerParent.UpdateVillagerCondition` (`self.VillagerParentRef`) false))
  (return _villagercondition))

(fn `DebugVillagerCondition`)

(fn `GetCharacterFromCurrentRow`
  (returns (CharacterName :type String))
  (return (`.CharacterName_10_A9D204DA4B87C77FC74CAABEDEF3AD6A` (break `/Game/FarmingDungeon/Blueprints/Manager/ST_DialogueRowDatas` (`self.CurrentDialogueRow`)))))

(fn `GetCurrentDialogueRow`
  (returns (RowData :type "/Game/FarmingDungeon/Blueprints/Manager/ST_DialogueRowDatas Structure"))
  (`self.CheckVillagerState`)
  (bind _returnvalue (`|GetDataTableRow` (`self.DialogueDataTable`) (`KismetStringLibrary.Conv_StringToName` (`KismetStringLibrary.Conv_IntToString` (`self.CurrentRowNumber`))))
    (:`then`
      (bind _output_get (set `self.CurrentDialogueRow` _returnvalue))
      (set `self.CurrentDialogueRowChoices` (`.Choices_15_2CBC833044FBB4FC0B43BF96BEB6CF77` (break `/Game/FarmingDungeon/Blueprints/Manager/ST_DialogueRowDatas` _output_get)))
      (return (`self.CurrentDialogueRow`)))))

(fn `GetDialogueTextFromCurrentRow`
  (returns (ChoicesText :type "Array of String") (DialogueText :type String))
  (if (`KismetArrayLibrary.Array_IsNotEmpty` (`.Choices_15_2CBC833044FBB4FC0B43BF96BEB6CF77` (break `/Game/FarmingDungeon/Blueprints/Manager/ST_DialogueRowDatas` (`self.CurrentDialogueRow`))))
    (bind _dialoguetextchoices (`self.ReadAllChoices`)))
  (return _dialoguetextchoices (`.DialogueText_8_E87BDCCB4F76D3270BB994B820CB55EB` (break `/Game/FarmingDungeon/Blueprints/Manager/ST_DialogueRowDatas` (`self.CurrentDialogueRow`)))))

(fn `IsDialogueFinished`
  (params (IndexOfChoice :type Integer))
  (returns (IsFinished :type Boolean))
  (bind _returnvalue (or (`.IsDialogueFinished_27_D24640884F6A1E8DFE78E5940F615D0E` (break `/Game/FarmingDungeon/Blueprints/Manager/ST_DialogueRowDatas` (`self.CurrentDialogueRow`))) (`.IsDialogueFinished_18_4E79DB7C456E15D20C00A283C790B76D` (break `/Game/FarmingDungeon/Blueprints/Manager/ST_DialogueChoices` (`|GetArrayItem` (`self.CurrentDialogueRowChoices`) IndexOfChoice)))))
  (if _returnvalue
    (bind _villagercondition (`self.CheckVillagerState`))
    (if (not _villagercondition)
      (set `self.CurrentRowNumber` (`.NextRow_9_55C368164B14ED92516079A0C993B082` (break `/Game/FarmingDungeon/Blueprints/Manager/ST_DialogueRowDatas` (`self.CurrentDialogueRow`))))
      (`self.CheckTriggerMovement`)
      (bind _asbp_isabelle (cast `/Game/FarmingDungeon/Blueprints/Characters/Villageois/BP_Isabelle` (`self.VillagerParentRef`))
        (:`then`
          (`/Game/FarmingDungeon/Blueprints/Characters/Villageois/BP_Isabelle.Tuto` _asbp_isabelle))
        (:`CastFailed`
          _))
      (return _returnvalue))
    (else
      (return _returnvalue))))

(fn `ReadAllChoices`
  (returns (DialogueTextChoices :type "Array of String"))
  (locals (ListAllChoices :type "Array of String"))
  (for _array_element (`self.CurrentDialogueRowChoices`)
    (`KismetArrayLibrary.Array_Add` (`local.ListAllChoices`) (`.DialogueText_8_E87BDCCB4F76D3270BB994B820CB55EB` (break `/Game/FarmingDungeon/Blueprints/Manager/ST_DialogueChoices` _array_element))))
  (return (`local.ListAllChoices`)))

(fn `ReadNextRow`
  (params (IndexOfChoice :type Integer))
  (`|ExecutionSequence`
    (:`then_0`
      (bind _villagercondition (`self.CheckVillagerState`))
      (if _villagercondition
        ;[1 1 1] Change la prochaine ligne en fonction de la condition du villageois
        (if (`KismetArrayLibrary.Array_IsEmpty` (`self.CurrentDialogueRowChoices`))
          (set `self.CurrentRowNumber` (`.NextRowByCondition_24_4E3BC43C476CEED0D19D07AC061603EF` (break `/Game/FarmingDungeon/Blueprints/Manager/ST_DialogueRowDatas` (`self.CurrentDialogueRow`))))
          (else
            (set `self.CurrentRowNumber` (`.NextRowByCondition_16_659B09034AD7CCBF2BF0ECAC98D3D4A9` (break `/Game/FarmingDungeon/Blueprints/Manager/ST_DialogueChoices` (`|GetArrayItem` (`self.CurrentDialogueRowChoices`) IndexOfChoice))))))
        (else
          ;[1 1 1] Lis la prochaine ligne de la Data table
          (if (`KismetArrayLibrary.Array_IsEmpty` (`self.CurrentDialogueRowChoices`))
            (set `self.CurrentRowNumber` (`.NextRow_9_55C368164B14ED92516079A0C993B082` (break `/Game/FarmingDungeon/Blueprints/Manager/ST_DialogueRowDatas` (`self.CurrentDialogueRow`))))
            (else
              (set `self.CurrentRowNumber` (`.NextRow_9_55C368164B14ED92516079A0C993B082` (break `/Game/FarmingDungeon/Blueprints/Manager/ST_DialogueChoices` (`|GetArrayItem` (`self.CurrentDialogueRowChoices`) IndexOfChoice)))))))))
    (:`then_1`
      ;[0.3262 0 0.4281] Fin
      (`self.GetCurrentDialogueRow`))))

(fn `ResetDialogueData`
  (set `self.CurrentRowNumber` 0))