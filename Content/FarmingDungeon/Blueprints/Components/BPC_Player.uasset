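; Player component that switches the local player between gameplay and menu input modes.
; SetMenuInput shows the mouse cursor and swaps the Enhanced Input mapping context from IMC_Game to IMC_Menu.
; SetGameInput does the reverse, hiding the cursor and restoring IMC_Game.
; Both act on player controller 0, and the event graph holds no active logic.
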(fn `SetGameInput`
  (bind _returnvalue (`GameplayStatics.GetPlayerController` 0))
  (bind _returnvalue_2 (pcsubsystem `EnhancedInputLocalPlayerSubsystem` _returnvalue))
  (set `PlayerController.bShowMouseCursor` false _returnvalue)
  (`EnhancedInputSubsystemInterface.RemoveMappingContext` _returnvalue_2 "/Game/FarmingDungeon/Blueprints/Manager/Inputs/InputActions/IMC_Menu.IMC_Menu" (struct))
  (`EnhancedInputSubsystemInterface.AddMappingContext` _returnvalue_2 "/Game/FarmingDungeon/Blueprints/Manager/Inputs/InputActions/IMC_Game.IMC_Game" 0 (struct)))

(fn `SetMenuInput`
  (bind _returnvalue (`GameplayStatics.GetPlayerController` 0))
  (bind _returnvalue_2 (pcsubsystem `EnhancedInputLocalPlayerSubsystem` _returnvalue))
  (set `PlayerController.bShowMouseCursor` true _returnvalue)
  (`EnhancedInputSubsystemInterface.RemoveMappingContext` _returnvalue_2 "/Game/FarmingDungeon/Blueprints/Manager/Inputs/InputActions/IMC_Game.IMC_Game" (struct))
  (`EnhancedInputSubsystemInterface.AddMappingContext` _returnvalue_2 "/Game/FarmingDungeon/Blueprints/Manager/Inputs/InputActions/IMC_Menu.IMC_Menu" 0 (struct)))