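; BPC_Loot is an actor component that adds its loot class to the player inventory held in BP_GameInstance.
; CheckPositionInventory looks for a matching slot below MaxStack, falling back to the first zero-count slot through CheckEmptySlot.
; AddInventory writes the class and increments the count in two parallel arrays, with debug prints.
; A separate DestroyparentActor function destroys the owning actor; nothing in this component calls it.
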(event `self.ReceiveBeginPlay`
  (bind _asbp_game_instance (cast `/Game/FarmingDungeon/Blueprints/Manager/BP_GameInstance` (`GameplayStatics.GetGameInstance`)))
  (set `self.Ref_BP_GameInstance` _asbp_game_instance))

(fn `AddInventory`
  (params (Index :type Integer) (ClassLoot :type "/Game/FarmingDungeon/Blueprints/Manager/E_Items Enum" :default "NewEnumerator0"))
  (bind _ref_bp_gameinstance (`self.Ref_BP_GameInstance`))
  (bind _nombreitem_inventaire_player (`/Game/FarmingDungeon/Blueprints/Manager/BP_GameInstance.NombreItem_Inventaire_Player` _ref_bp_gameinstance))
  (bind _returnvalue (+ (`|GetArrayItem` _nombreitem_inventaire_player Index) 1))
  (`KismetSystemLibrary.PrintString` "JE SUIS CENSE FONCTIONNER" true true (struct :`R` 0.893898 :`G` 0.488704 :`B` 1.0 :`A` 1.0))
  (`KismetArrayLibrary.Array_Set` (`/Game/FarmingDungeon/Blueprints/Manager/BP_GameInstance.Inventaire_Player` _ref_bp_gameinstance) Index ClassLoot)
  (`KismetSystemLibrary.PrintString` (`KismetStringLibrary.Conv_IntToString` _returnvalue))
  (`KismetArrayLibrary.Array_Set` _nombreitem_inventaire_player Index _returnvalue)
  (set `self.IsAdded` true))

(fn `CheckEmptySlot`
  (for (_array_element _array_index) (`/Game/FarmingDungeon/Blueprints/Manager/BP_GameInstance.NombreItem_Inventaire_Player` (`self.Ref_BP_GameInstance`))
    (if (<= _array_element 0)
      (bind _output_get (set `self.Index` _array_index))
      (`self.AddInventory` _output_get (`self.ClassName`))
      (break))))

(fn `CheckPositionInventory`
  (`KismetSystemLibrary.PrintString` "Hello" true true (struct :`R` 1.0 :`G` 0.448468 :`A` 1.0))
  (set `self.IsAdded` false)
  (for (_array_element _array_index) (`/Game/FarmingDungeon/Blueprints/Manager/BP_GameInstance.Inventaire_Player` (`self.Ref_BP_GameInstance`))
    (if (`|EnumEquality` _array_element (`self.ClassName`))
      (bind _ismaxstack (`self.CheckStack` _array_index (`self.MaxStack`)))
      (if (not _ismaxstack)
        (bind _output_get (set `self.Index` _array_index))
        (`self.AddInventory` _output_get (`self.ClassName`))
        (break))))
  (if (not (`self.IsAdded`))
    (`self.CheckEmptySlot`)))

(fn `CheckStack`
  (params (Index :type Integer) (MaxStack :type Integer))
  (returns (IsMaxStack :type Boolean))
  (return (>= (`|GetArrayItem` (`/Game/FarmingDungeon/Blueprints/Manager/BP_GameInstance.NombreItem_Inventaire_Player` (`self.Ref_BP_GameInstance`)) Index) MaxStack)))

(fn `DestroyparentActor`
  (`Actor.K2_DestroyActor` (`self.GetOwner`)))