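; BPC_PV is a health component (PV, hit points) that tracks damage and death for its owner, with extra support for the player.
; GetHit subtracts attack damage from PV and calls the EDMort death dispatcher at zero or below.
; UpdatePVPlayer copies PV, floored at zero when depleted, into the GameInstance's PVPlayer, triggers a player HUD update and also signals death at zero.
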(fn `Get_Hit`
  (params (Attack :type "Float (double-precision)"))
  (bind _output_get (set `self.PV` (- (`self.PV`) Attack)))
  (if (<= _output_get 0.0)
    (`self.ED_Mort`)))

(fn `Update_PVPlayer`
  (params (GameInstance :type "/Game/FarmingDungeon/Blueprints/Manager/BP_GameInstance Object Reference"))
  (bind _pv (`self.PV`))
  (if (<= _pv 0.0)
    (set `/Game/FarmingDungeon/Blueprints/Manager/BP_GameInstance.PV_Player` 0.0 GameInstance)
    (`self.UpdateHUDPlayer`)
    (`self.ED_Mort`)
    (else
      (set `/Game/FarmingDungeon/Blueprints/Manager/BP_GameInstance.PV_Player` _pv GameInstance)
      ;[1 0.943 0.172] ilian
      (`self.UpdateHUDPlayer`))))