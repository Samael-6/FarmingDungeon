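; BP_DialogueBox is a trigger volume actor that starts a villager interaction when the player walks into it.
; On BeginPlay, Activate sets Box1 collision on or off according to the Active flag.
; When a BP_Player begins overlapping Box while Active is set, it calls OnInteract on the referenced villager.
; A forward-vector facing check is present but unused.
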(event `self.ReceiveBeginPlay`
  (`self.Activate`))

(event `self.Box.OnComponentBeginOverlap`
  (params (OverlappedComponent :type "PrimitiveComponent Object Reference") (OtherActor :type "Actor Object Reference") (OtherComp :type "PrimitiveComponent Object Reference") (OtherBodyIndex :type Integer) (bFromSweep :type Boolean) (SweepResult :type "HitResult Structure (by ref)"))
  (bind _asbp_player (cast `/Game/FarmingDungeon/Blueprints/Characters/BP_Player` OtherActor))
  (if (`self.Active`)
    (`/Game/FarmingDungeon/Blueprints/Characters/Villageois/BP_VillagerParent.OnInteract` (`self.VillagerRef`) _asbp_player)))

(fn `Activate`
  (if (`self.Active`)
    (`PrimitiveComponent.SetCollisionEnabled` (`self.Box1`) "QueryAndPhysics")
    (else
      (`PrimitiveComponent.SetCollisionEnabled` (`self.Box1`) "NoCollision"))))

(fn `UserConstructionScript`)