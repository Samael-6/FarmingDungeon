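; BP_Poule is a chicken character that wanders on its own.
; On BeginPlay, ChangeRotation gives Arrow1 a random yaw and repeats itself after random delays while Canrot is true.
; Tick feeds the arrow's forward vector, scaled by Speed, into movement input.
; A short Camera-channel line trace from the mesh along that direction triggers an immediate new heading when it hits something.
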(event `ChangeRotation`
  (`SceneComponent.K2_SetWorldRotation` (`self.Arrow1`) (`KismetMathLibrary.MakeRotator` 0.0 0.0 (`KismetMathLibrary.RandomFloatInRange` -180.0 180.0)) false false)
  (set `self.canrot` true)
  (`KismetSystemLibrary.Delay` (`KismetMathLibrary.RandomFloatInRange` 2.0 15.0))
  (if (`self.canrot`)
    (`self.ChangeRotation`)))

(event `self.ReceiveBeginPlay`
  (`self.ChangeRotation`))

(event `self.ReceiveTick`
  (params (DeltaSeconds :type "Float (single-precision)"))
  (bind _returnvalue (`SceneComponent.K2_GetComponentLocation` (`self.Mesh`)))
  (`self.AddMovementInput` (* (`SceneComponent.GetForwardVector` (`self.Arrow1`)) (`self.Speed`)))
  (bind (_outhit _returnvalue_2) (`KismetSystemLibrary.LineTraceSingle` _returnvalue (+ _returnvalue (* (`SceneComponent.GetForwardVector` (`self.Arrow1`)) 150.0)) "TraceTypeQuery2"))
  (if _returnvalue_2
    (set `self.canrot` false)
    (`self.ChangeRotation`)))

(fn `UserConstructionScript`)