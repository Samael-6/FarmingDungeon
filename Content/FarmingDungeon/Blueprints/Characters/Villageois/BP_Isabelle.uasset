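; Villager NPC Isabelle, who opens the game's dialogue on start until the tutorial is finished, then starts from a post-tutorial spot.
; Her quest state and condition come from the Game Instance, and a nested flag check picks her dialogue row from the furthest villager quest progress and owned weapons.
; Her Tuto function advances the tutorial manager around farm, fight and storage steps.
; One dialogue row also displays the village estrade.
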(event `Start`
  (`parent.ReceiveBeginPlay`)
  (set `self.E_VillagerName` "NewEnumerator0")
  (set `self.MapsOfCamView` (`self.IsabelleCamMaps`))
  (add `self.DisplayAssetsInWorld` (delegate `DisplayEstrade`))
  (set `self.HasStartedQuest` true)
  (set `self.VillagerCondition` (`/Game/FarmingDungeon/Blueprints/Manager/BP_GameInstance.IsabelleCondition` (`/Game/FarmingDungeon/Blueprints/Components/BPC_Dialogue.GameInstanceRef` (`self.BPC_Dialogue`))))
  (set `self.HasFinishedQuest` (`/Game/FarmingDungeon/Blueprints/Manager/BP_GameInstance.HasFinishedIsabelleQuest` (`/Game/FarmingDungeon/Blueprints/Components/BPC_Dialogue.GameInstanceRef` (`self.BPC_Dialogue`))))
  (`KismetSystemLibrary.DelayUntilNextTick`)
  (if (`/Game/FarmingDungeon/Blueprints/Manager/BP_GameInstance.HasFinishedTuto` (`/Game/FarmingDungeon/Blueprints/Components/BPC_Dialogue.GameInstanceRef` (`self.BPC_Dialogue`)))
    (`self.K2_SetActorTransform` (`self.GetTransform` (`self.StartingPointAfterTuto`)))
    (else
      ;[1 1 1] Start with dialogue
      (`/Game/FarmingDungeon/Blueprints/Interfaces/BPI_Interact.OnInteract` (`/Game/FarmingDungeon/Blueprints/Manager/BP_GameInstance.Bp_PlayerRef` (`self.As BP Game Instance`))))))

(event `self.ReceiveBeginPlay`)

(event `self.UpdateVillagerCondition`
  (params (ResetValue :type Boolean))
  (bind _output_get (set `/Game/FarmingDungeon/Blueprints/Manager/BP_GameInstance.IsabelleCondition` ResetValue (`/Game/FarmingDungeon/Blueprints/Components/BPC_Dialogue.GameInstanceRef` (`self.BPC_Dialogue`))))
  (bind _output_get_2 (set `self.VillagerCondition` _output_get)))

(event `DisplayEstrade`
  (if (== (`/Game/FarmingDungeon/Blueprints/Components/BPC_Dialogue.CurrentRowNumber` (`self.BPC_Dialogue`)) 25)
    (`/Game/FarmingDungeon/Blueprints/Manager/GameModes/BP_GM_Village.DisplayEstrade` (`self.As BP GM Village`) true)))

(event `self.UpdateFinishedQuest`
  (set `self.HasFinishedQuest` (`/Game/FarmingDungeon/Blueprints/Manager/BP_GameInstance.HasFinishedIsabelleQuest` (`/Game/FarmingDungeon/Blueprints/Components/BPC_Dialogue.GameInstanceRef` (`self.BPC_Dialogue`)))))

(event `self.CheckIfQuestSTarted`
  (if (`/Game/FarmingDungeon/Blueprints/Manager/BP_GameInstance.HasFinishedVladimirQuest` (`/Game/FarmingDungeon/Blueprints/Components/BPC_Dialogue.GameInstanceRef` (`self.BPC_Dialogue`)))
    (set `/Game/FarmingDungeon/Blueprints/Components/BPC_Dialogue.CurrentRowNumber` 35 (`self.BPC_Dialogue`))
    (elif (`/Game/FarmingDungeon/Blueprints/Manager/BP_GameInstance.HasStartedVladimir` (`/Game/FarmingDungeon/Blueprints/Components/BPC_Dialogue.GameInstanceRef` (`self.BPC_Dialogue`)))
      (bind _hasweapon (`/Game/FarmingDungeon/Blueprints/Manager/BP_GameInstance.CheckIfHasWeapon` (`/Game/FarmingDungeon/Blueprints/Components/BPC_Dialogue.GameInstanceRef` (`self.BPC_Dialogue`)) "NewEnumerator2"))
      (if _hasweapon
        (set `/Game/FarmingDungeon/Blueprints/Components/BPC_Dialogue.CurrentRowNumber` 34 (`self.BPC_Dialogue`))
        (else
          (set `/Game/FarmingDungeon/Blueprints/Components/BPC_Dialogue.CurrentRowNumber` 33 (`self.BPC_Dialogue`))))
      (elif (`/Game/FarmingDungeon/Blueprints/Manager/BP_GameInstance.HasFinishedMaryQuest` (`/Game/FarmingDungeon/Blueprints/Components/BPC_Dialogue.GameInstanceRef` (`self.BPC_Dialogue`)))
        (set `/Game/FarmingDungeon/Blueprints/Components/BPC_Dialogue.CurrentRowNumber` 32 (`self.BPC_Dialogue`))
        (elif (`/Game/FarmingDungeon/Blueprints/Manager/BP_GameInstance.HasStartedMary` (`/Game/FarmingDungeon/Blueprints/Components/BPC_Dialogue.GameInstanceRef` (`self.BPC_Dialogue`)))
          (bind _hasweapon_2 (`/Game/FarmingDungeon/Blueprints/Manager/BP_GameInstance.CheckIfHasWeapon` (`/Game/FarmingDungeon/Blueprints/Components/BPC_Dialogue.GameInstanceRef` (`self.BPC_Dialogue`)) "NewEnumerator1"))
          (if _hasweapon_2
            (set `/Game/FarmingDungeon/Blueprints/Components/BPC_Dialogue.CurrentRowNumber` 31 (`self.BPC_Dialogue`))
            (else
              (set `/Game/FarmingDungeon/Blueprints/Components/BPC_Dialogue.CurrentRowNumber` 30 (`self.BPC_Dialogue`))))
          (elif (`/Game/FarmingDungeon/Blueprints/Manager/BP_GameInstance.HasFinishedJeanEudeQuest` (`/Game/FarmingDungeon/Blueprints/Components/BPC_Dialogue.GameInstanceRef` (`self.BPC_Dialogue`)))
            (set `/Game/FarmingDungeon/Blueprints/Components/BPC_Dialogue.CurrentRowNumber` 29 (`self.BPC_Dialogue`))
            (elif (`/Game/FarmingDungeon/Blueprints/Manager/BP_GameInstance.HasStartedJeanEude` (`/Game/FarmingDungeon/Blueprints/Components/BPC_Dialogue.GameInstanceRef` (`self.BPC_Dialogue`)))
              (set `/Game/FarmingDungeon/Blueprints/Components/BPC_Dialogue.CurrentRowNumber` 28 (`self.BPC_Dialogue`))
              (elif (`/Game/FarmingDungeon/Blueprints/Manager/BP_GameInstance.HasFinishedIsabelleQuest` (`/Game/FarmingDungeon/Blueprints/Components/BPC_Dialogue.GameInstanceRef` (`self.BPC_Dialogue`)))
                (set `/Game/FarmingDungeon/Blueprints/Components/BPC_Dialogue.CurrentRowNumber` 28 (`self.BPC_Dialogue`))
                (elif (`/Game/FarmingDungeon/Blueprints/Manager/BP_GameInstance.HasFinishedTuto` (`/Game/FarmingDungeon/Blueprints/Components/BPC_Dialogue.GameInstanceRef` (`self.BPC_Dialogue`)))
                  (set `/Game/FarmingDungeon/Blueprints/Components/BPC_Dialogue.CurrentRowNumber` 24 (`self.BPC_Dialogue`))
                  (else
                    (set `/Game/FarmingDungeon/Blueprints/Components/BPC_Dialogue.CurrentRowNumber` 0 (`self.BPC_Dialogue`))))))))))))

(fn `IsInteractible`
  (returns (Interactable :type Boolean))
  (return true))

(fn `Tuto`
  (bind _bpc_tutorialmanager (`/Game/FarmingDungeon/Blueprints/Quest/Tutorial/BP_TutorialManager.BPC_TutorialManager` (`self.TutoManagerRef`)))
  (bind _asbp_player (cast `/Game/FarmingDungeon/Blueprints/Characters/BP_Player` (`GameplayStatics.GetPlayerPawn` 0)))
  (if (and (`/Game/FarmingDungeon/Blueprints/Quest/Tutorial/BPC_TutorialManager.HasEnterFarm` (`/Game/FarmingDungeon/Blueprints/Quest/Tutorial/BP_TutorialManager.BPC_TutorialManager` (`self.TutoManagerRef`))) (not (`/Game/FarmingDungeon/Blueprints/Quest/Tutorial/BPC_TutorialManager.StartFight` (`/Game/FarmingDungeon/Blueprints/Quest/Tutorial/BP_TutorialManager.BPC_TutorialManager` (`self.TutoManagerRef`)))))
    (set `/Game/FarmingDungeon/Blueprints/Quest/Tutorial/BPC_TutorialManager.StartFight` true (`/Game/FarmingDungeon/Blueprints/Quest/Tutorial/BP_TutorialManager.BPC_TutorialManager` (`self.TutoManagerRef`)))
    (`/Game/FarmingDungeon/Blueprints/Quest/Tutorial/BPC_TutorialManager.UpdateState` (`/Game/FarmingDungeon/Blueprints/Quest/Tutorial/BP_TutorialManager.BPC_TutorialManager` (`self.TutoManagerRef`)) _asbp_player :!label _label)
    (elif (`/Game/FarmingDungeon/Blueprints/Quest/Tutorial/BPC_TutorialManager.HasFinishFight` _bpc_tutorialmanager)
      (goto _label)
      (elif (`/Game/FarmingDungeon/Blueprints/Quest/Tutorial/BPC_TutorialManager.HasStockedObject` _bpc_tutorialmanager)
        (set `/Game/FarmingDungeon/Blueprints/Quest/Tutorial/BPC_TutorialManager.HasFinishedTalkingToIsabelle` true _bpc_tutorialmanager)
        (goto _label)))))

(fn `UserConstructionScript`
  (`parent.UserConstructionScript`))