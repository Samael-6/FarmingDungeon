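; BP_Vladimir is the villager NPC Vladimir, built on a parent class and always interactible.
; On BeginPlay it creates his services widget, stores it as the services HUD reference, and loads his villager condition from the Game Instance through the dialogue component.
; Condition updates are written to the Game Instance, copied back to the local variable and printed as debug output.
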(event `self.ReceiveBeginPlay`
  (`parent.ReceiveBeginPlay`)
  (bind _returnvalue (`|CreateWidget` "/Game/FarmingDungeon/Blueprints/Widgets/WBP_VladimirServices.WBP_VladimirServices_C"))
  (set `self.HUDServicesRef` _returnvalue)
  (set `self.VillagerCondition` (`/Game/FarmingDungeon/Blueprints/Manager/BP_GameInstance.VladimirCondition` (`/Game/FarmingDungeon/Blueprints/Components/BPC_Dialogue.GameInstanceRef` (`self.BPC_Dialogue`)))))

(event `self.UpdateVillagerCondition`
  (params (ResetValue :type Boolean))
  (bind _output_get (set `/Game/FarmingDungeon/Blueprints/Manager/BP_GameInstance.VladimirCondition` ResetValue (`/Game/FarmingDungeon/Blueprints/Components/BPC_Dialogue.GameInstanceRef` (`self.BPC_Dialogue`))))
  (bind _output_get_2 (set `self.VillagerCondition` _output_get))
  (`KismetSystemLibrary.PrintString` (`KismetStringLibrary.Conv_BoolToString` _output_get_2)))

(fn `IsInteractible`
  (returns (Interactable :type Boolean))
  (return true))

(fn `UserConstructionScript`
  (`parent.UserConstructionScript`))