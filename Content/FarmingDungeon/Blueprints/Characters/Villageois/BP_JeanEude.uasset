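; BP_JeanEude is the villager Jean Eude, an always-interactible NPC with dialogue, a quest and a services menu.
; On BeginPlay it creates its services widget and restores villager condition and quest progress from the Game Instance, reached through the dialogue component.
; Update events sync condition and quest flags with that Game Instance.
; The dialogue's starting row depends on whether his quest has started and Isabelle's quest is finished.
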(event `self.ReceiveBeginPlay`
  (bind _gameinstanceref (`/Game/FarmingDungeon/Blueprints/Components/BPC_Dialogue.GameInstanceRef` (`self.BPC_Dialogue`)))
  (`parent.ReceiveBeginPlay`)
  (set `self.E_VillagerName` "NewEnumerator1")
  (bind _returnvalue (`|CreateWidget` "/Game/FarmingDungeon/Blueprints/Widgets/WBP_JeanEudeServices.WBP_JeanEudeServices_C"))
  (set `/Game/FarmingDungeon/Blueprints/Widgets/WBP_JeanEudeServices.VillagerRef` self _returnvalue)
  (set `self.HUDServicesRef` _returnvalue)
  (set `self.VillagerCondition` (`/Game/FarmingDungeon/Blueprints/Manager/BP_GameInstance.JeanEudeCondition` _gameinstanceref))
  (set `self.HasStartedQuest` (`/Game/FarmingDungeon/Blueprints/Manager/BP_GameInstance.HasStartedJeanEude` _gameinstanceref))
  (set `self.HasFinishedQuest` (`/Game/FarmingDungeon/Blueprints/Manager/BP_GameInstance.HasFinishedJeanEudeQuest` (`/Game/FarmingDungeon/Blueprints/Components/BPC_Dialogue.GameInstanceRef` (`self.BPC_Dialogue`))))
  (bind _nameofvillagerforquest (`/Game/FarmingDungeon/Blueprints/Manager/BP_GameInstance.GetGameState` (`/Game/FarmingDungeon/Blueprints/Components/BPC_Dialogue.GameInstanceRef` (`self.BPC_Dialogue`))))
  (if (`|EnumEquality` _nameofvillagerforquest "NewEnumerator1")
    (set `self.NumberOfItemsGiven` (`/Game/FarmingDungeon/Blueprints/Manager/BP_GameInstance.NumberOfItemsGivenForQuest` (`/Game/FarmingDungeon/Blueprints/Components/BPC_Dialogue.GameInstanceRef` (`self.BPC_Dialogue`))))))

(event `self.UpdateVillagerCondition`
  (params (ResetValue :type Boolean))
  (bind _output_get (set `/Game/FarmingDungeon/Blueprints/Manager/BP_GameInstance.JeanEudeCondition` ResetValue (`/Game/FarmingDungeon/Blueprints/Components/BPC_Dialogue.GameInstanceRef` (`self.BPC_Dialogue`))))
  (bind _output_get_2 (set `self.VillagerCondition` _output_get)))

(event `self.ReceiveTick`
  (params (DeltaSeconds :type "Float (single-precision)")))

(event `self.UpdateStartedQuest`
  (params (Value :type Boolean))
  (bind _output_get (set `self.HasStartedQuest` Value))
  (set `/Game/FarmingDungeon/Blueprints/Manager/BP_GameInstance.HasStartedJeanEude` _output_get (`/Game/FarmingDungeon/Blueprints/Components/BPC_Dialogue.GameInstanceRef` (`self.BPC_Dialogue`))))

(event `self.UpdateFinishedQuest`
  (set `self.HasFinishedQuest` (`/Game/FarmingDungeon/Blueprints/Manager/BP_GameInstance.HasFinishedJeanEudeQuest` (`/Game/FarmingDungeon/Blueprints/Components/BPC_Dialogue.GameInstanceRef` (`self.BPC_Dialogue`)))))

(event `self.CheckIfQuestSTarted`
  (if (`self.HasStartedQuest`)
    (set `/Game/FarmingDungeon/Blueprints/Components/BPC_Dialogue.CurrentRowNumber` 8 (`self.BPC_Dialogue`))
    (elif (`/Game/FarmingDungeon/Blueprints/Manager/BP_GameInstance.HasFinishedIsabelleQuest` (`/Game/FarmingDungeon/Blueprints/Components/BPC_Dialogue.GameInstanceRef` (`self.BPC_Dialogue`)))
      (set `/Game/FarmingDungeon/Blueprints/Components/BPC_Dialogue.CurrentRowNumber` 3 (`self.BPC_Dialogue`))
      (else
        (set `/Game/FarmingDungeon/Blueprints/Components/BPC_Dialogue.CurrentRowNumber` 8 (`self.BPC_Dialogue`))))))

(fn `IsInteractible`
  (returns (Interactable :type Boolean))
  (return true))

(fn `UserConstructionScript`
  (`parent.UserConstructionScript`))