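; Parent Blueprint for villagers, an always-interactible character that runs a dialogue with the player.
; It creates a WBP_DialogueUI on BeginPlay with a back-reference to itself, then fills it with speaker and text rows read from BPCDialogue.
; Interacting shows the dialogue and cursor and swaps Enhanced Input from IMC_Game to IMC_Menu.
; Update advances rows until the dialogue finishes, then Deactivate removes the widget and restores game input.
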(event `self.ReceiveBeginPlay`
  (bind _returnvalue (`|CreateWidget` "/Game/FarmingDungeon/Blueprints/Widgets/WBP_DialogueUI.WBP_DialogueUI_C"))
  (bind _output_get (set `self.DialogueHUDRef` _returnvalue))
  (set `/Game/FarmingDungeon/Blueprints/Widgets/WBP_DialogueUI.VillageoisRef` self _output_get))

(event `Activate`
  (`/Game/FarmingDungeon/Blueprints/Components/BPC_Dialogue.GetCurrentDialogueRow` (`self.BPC_Dialogue`))
  (bind _charactername (`/Game/FarmingDungeon/Blueprints/Components/BPC_Dialogue.GetCharacterFromCurrentRow` (`self.BPC_Dialogue`)))
  (bind _dialoguetext (`/Game/FarmingDungeon/Blueprints/Components/BPC_Dialogue.GetDialogueTextFromCurrentRow` (`self.BPC_Dialogue`)))
  (`/Game/FarmingDungeon/Blueprints/Widgets/WBP_DialogueUI.UpdateDialogueText` (`self.DialogueHUDRef`) _charactername _dialoguetext)
  (`UserWidget.AddToPlayerScreen` (`self.DialogueHUDRef`) 0))

(event `Update`
  (bind _isfinished (`/Game/FarmingDungeon/Blueprints/Components/BPC_Dialogue.IsDialogueFinished` (`self.BPC_Dialogue`)))
  (if _isfinished
    (`self.Deactivate`)
    (else
      (`/Game/FarmingDungeon/Blueprints/Components/BPC_Dialogue.ReadNextRow` (`self.BPC_Dialogue`))
      (bind _charactername (`/Game/FarmingDungeon/Blueprints/Components/BPC_Dialogue.GetCharacterFromCurrentRow` (`self.BPC_Dialogue`)))
      (bind _dialoguetext (`/Game/FarmingDungeon/Blueprints/Components/BPC_Dialogue.GetDialogueTextFromCurrentRow` (`self.BPC_Dialogue`)))
      (`/Game/FarmingDungeon/Blueprints/Widgets/WBP_DialogueUI.UpdateDialogueText` (`self.DialogueHUDRef`) _charactername _dialoguetext))))

(event `Deactivate`
  (bind _returnvalue (pcsubsystem `EnhancedInputLocalPlayerSubsystem` (`GameplayStatics.GetPlayerController` 0)))
  (`Widget.RemoveFromParent` (`self.DialogueHUDRef`))
  (message `EnhancedInputSubsystemInterface.AddMappingContext` _returnvalue "/Game/FarmingDungeon/Blueprints/Manager/Inputs/InputActions/IMC_Game.IMC_Game" 0 (struct))
  (message `EnhancedInputSubsystemInterface.RemoveMappingContext` _returnvalue "/Game/FarmingDungeon/Blueprints/Manager/Inputs/InputActions/IMC_Menu.IMC_Menu" (struct))
  (set `PlayerController.bShowMouseCursor` false (`GameplayStatics.GetPlayerController` 0)))

(event `/Game/FarmingDungeon/Blueprints/Interfaces/BPI_Interact.OnInteract`
  (params (Player :type "/Game/FarmingDungeon/Blueprints/Characters/BP_Player Object Reference"))
  (bind _returnvalue (pcsubsystem `EnhancedInputLocalPlayerSubsystem` (`GameplayStatics.GetPlayerController` 0)))
  ;[1 1 1] Comment
  (`self.Activate`)
  (message `EnhancedInputSubsystemInterface.AddMappingContext` _returnvalue "/Game/FarmingDungeon/Blueprints/Manager/Inputs/InputActions/IMC_Menu.IMC_Menu" 0 (struct))
  (message `EnhancedInputSubsystemInterface.RemoveMappingContext` _returnvalue "/Game/FarmingDungeon/Blueprints/Manager/Inputs/InputActions/IMC_Game.IMC_Game" (struct))
  (set `PlayerController.bShowMouseCursor` true (`GameplayStatics.GetPlayerController` 0)))

(fn `IsInteractible`
  (returns (Interactable :type Boolean))
  (return true))

(fn `UserConstructionScript`)