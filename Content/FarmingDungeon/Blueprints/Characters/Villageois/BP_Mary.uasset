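; BP_Mary is the villager Mary, an always-interactible NPC with a dialogue component and her own services widget.
; On BeginPlay it creates the widget and restores her condition, quest flag and given-item counts from the game instance.
; Tutorial and quest flags there select the starting dialogue row, and her quest is flagged as started once Jean Eude's is finished.
; Separate events re-check that unlock and save condition changes back to the game instance.
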(event `self.ReceiveBeginPlay`
  (bind _gameinstanceref (`/Game/FarmingDungeon/Blueprints/Components/BPC_Dialogue.GameInstanceRef` (`self.BPC_Dialogue`)))
  (`parent.ReceiveBeginPlay`)
  (bind _returnvalue (`|CreateWidget` "/Game/FarmingDungeon/Blueprints/Widgets/WBP_MaryServices.WBP_MaryServices_C"))
  (set `/Game/FarmingDungeon/Blueprints/Widgets/WBP_MaryServices.VillagerRef` self _returnvalue)
  (set `self.HUDServicesRef` _returnvalue)
  (set `self.VillagerCondition` (`/Game/FarmingDungeon/Blueprints/Manager/BP_GameInstance.MaryCondition` _gameinstanceref))
  (set `self.HasStartedQuest` (`/Game/FarmingDungeon/Blueprints/Manager/BP_GameInstance.HasStartedMary` _gameinstanceref))
  (bind _nameofvillagerforquest (`/Game/FarmingDungeon/Blueprints/Manager/BP_GameInstance.GetGameState` (`/Game/FarmingDungeon/Blueprints/Components/BPC_Dialogue.GameInstanceRef` (`self.BPC_Dialogue`))))
  (if (`KismetStringLibrary.EqualEqual_StrStr` _nameofvillagerforquest "Mary")
    (set `self.NumberOfItemsGiven` (`/Game/FarmingDungeon/Blueprints/Manager/BP_GameInstance.NumberOfItemsGivenForQuest` (`/Game/FarmingDungeon/Blueprints/Components/BPC_Dialogue.GameInstanceRef` (`self.BPC_Dialogue`))))
    (set `self.NumberItemGiven2Slot` (`/Game/FarmingDungeon/Blueprints/Manager/BP_GameInstance.NumberOfItemsGivenForQuest2Slot` (`/Game/FarmingDungeon/Blueprints/Components/BPC_Dialogue.GameInstanceRef` (`self.BPC_Dialogue`)))))
  (if (`/Game/FarmingDungeon/Blueprints/Manager/BP_GameInstance.HasFinishedTuto` _gameinstanceref)
    (if (`/Game/FarmingDungeon/Blueprints/Manager/BP_GameInstance.HasFinishedJeanEudeQuest` _gameinstanceref)
      (if (`self.HasStartedQuest`)
        (set `/Game/FarmingDungeon/Blueprints/Components/BPC_Dialogue.CurrentRowNumber` 7 (`self.BPC_Dialogue`) :!label _label)
        (else
          (set `/Game/FarmingDungeon/Blueprints/Manager/BP_GameInstance.HasStartedMary` true (`/Game/FarmingDungeon/Blueprints/Components/BPC_Dialogue.GameInstanceRef` (`self.BPC_Dialogue`)))
          (set `/Game/FarmingDungeon/Blueprints/Components/BPC_Dialogue.CurrentRowNumber` 2 (`self.BPC_Dialogue`))))
      (else
        (goto _label)))
    (else
      (set `/Game/FarmingDungeon/Blueprints/Components/BPC_Dialogue.CurrentRowNumber` 0 (`self.BPC_Dialogue`)))))

(event `self.UpdateVillagerCondition`
  (params (ResetValue :type Boolean))
  (bind _output_get (set `/Game/FarmingDungeon/Blueprints/Manager/BP_GameInstance.MaryCondition` ResetValue (`/Game/FarmingDungeon/Blueprints/Components/BPC_Dialogue.GameInstanceRef` (`self.BPC_Dialogue`))))
  (bind _output_get_2 (set `self.VillagerCondition` _output_get)))

(event `self.CheckIfQuestSTarted`
  (if (and (`/Game/FarmingDungeon/Blueprints/Manager/BP_GameInstance.HasFinishedJeanEudeQuest` (`/Game/FarmingDungeon/Blueprints/Components/BPC_Dialogue.GameInstanceRef` (`self.BPC_Dialogue`))) (not (`self.HasStartedQuest`)))
    (bind _output_get (set `/Game/FarmingDungeon/Blueprints/Manager/BP_GameInstance.HasStartedMary` true (`/Game/FarmingDungeon/Blueprints/Components/BPC_Dialogue.GameInstanceRef` (`self.BPC_Dialogue`))))
    (set `self.HasStartedQuest` _output_get)
    (set `/Game/FarmingDungeon/Blueprints/Components/BPC_Dialogue.CurrentRowNumber` 2 (`self.BPC_Dialogue`))
    (elif (`/Game/FarmingDungeon/Blueprints/Manager/BP_GameInstance.HasFinishedIsabelleQuest` (`/Game/FarmingDungeon/Blueprints/Components/BPC_Dialogue.GameInstanceRef` (`self.BPC_Dialogue`)))
      (set `/Game/FarmingDungeon/Blueprints/Components/BPC_Dialogue.CurrentRowNumber` 7 (`self.BPC_Dialogue`)))))

(fn `IsInteractible`
  (returns (Interactable :type Boolean))
  (return true))

(fn `UserConstructionScript`
  (`parent.UserConstructionScript`))