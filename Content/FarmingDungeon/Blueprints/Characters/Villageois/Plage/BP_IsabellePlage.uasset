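; Beach version of the villager Isabelle, an interactible NPC who also triggers the end-of-game fireworks cinematic.
; BeginPlay marks her quest started and syncs condition and completion from the GameInstance via the dialogue component.
; CINFireworks hides her, the player and HUD, reveals show actors, starts fireworks, sequence and audio, then displays credits.
; Tuto advances tutorial state; older dialogue-row selection, tutorial repositioning and main-menu return logic are disconnected.
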(event `Start`)

(event `self.ReceiveBeginPlay`
  (`parent.ReceiveBeginPlay`)
  (set `self.HasStartedQuest` true)
  (set `self.VillagerCondition` (`/Game/FarmingDungeon/Blueprints/Manager/BP_GameInstance.IsabelleCondition` (`/Game/FarmingDungeon/Blueprints/Components/BPC_Dialogue.GameInstanceRef` (`self.BPC_Dialogue`))))
  (set `self.HasFinishedQuest` (`/Game/FarmingDungeon/Blueprints/Manager/BP_GameInstance.HasFinishedIsabelleQuest` (`/Game/FarmingDungeon/Blueprints/Components/BPC_Dialogue.GameInstanceRef` (`self.BPC_Dialogue`)))))

(event `self.UpdateVillagerCondition`
  (params (ResetValue :type Boolean))
  (bind _output_get (set `/Game/FarmingDungeon/Blueprints/Manager/BP_GameInstance.IsabelleCondition` ResetValue (`/Game/FarmingDungeon/Blueprints/Components/BPC_Dialogue.GameInstanceRef` (`self.BPC_Dialogue`))))
  (set `self.VillagerCondition` _output_get))

(event `DisplayEstrade`
  (if (== (`/Game/FarmingDungeon/Blueprints/Components/BPC_Dialogue.CurrentRowNumber` (`self.BPC_Dialogue`)) 25)
    (`/Game/FarmingDungeon/Blueprints/Manager/GameModes/BP_GM_Village.DisplayEstrade` (`self.As BP GM Village`) true)))

(event `self.UpdateFinishedQuest`
  (set `self.HasFinishedQuest` (`/Game/FarmingDungeon/Blueprints/Manager/BP_GameInstance.HasFinishedIsabelleQuest` (`/Game/FarmingDungeon/Blueprints/Components/BPC_Dialogue.GameInstanceRef` (`self.BPC_Dialogue`)))))

(event `self.CheckIfQuestSTarted`
  (set `/Game/FarmingDungeon/Blueprints/Components/BPC_Dialogue.CurrentRowNumber` 0 (`self.BPC_Dialogue`)))

(event `CINFireworks`
  (`self.SetActorHiddenInGame` true)
  (bind _returnvalue (`GameplayStatics.GetActorOfClass` "/Game/FarmingDungeon/Blueprints/Characters/BP_Player.BP_Player_C"))
  (`self.DisableInput` _returnvalue (`GameplayStatics.GetPlayerController` 0))
  (`self.SetActorHiddenInGame` _returnvalue true)
  (`self.SetActorHiddenInGame` (`/Game/FarmingDungeon/Blueprints/Characters/BP_Player.Ref_ActualWeapon` _returnvalue) true)
  (`Widget.RemoveFromParent` (`/Game/FarmingDungeon/Blueprints/Characters/BP_Player.PlayerHUDRef` _returnvalue))
  (bind _outactors (`GameplayStatics.GetAllActorsOfClass` "/Game/FarmingDungeon/Blueprints/Actors/CINEMATICS/BP_ToShow.BP_ToShow_C"))
  (for _array_element _outactors
    (`self.SetActorHiddenInGame` _array_element false))
  (bind _outactors_2 (`GameplayStatics.GetAllActorsOfClass` "/Game/FarmingDungeon/Blueprints/Actors/CINEMATICS/BP_Fireworkd.BP_Fireworkd_C"))
  (for _array_element_2 _outactors_2
    (`ActorComponent.Activate` (`/Game/FarmingDungeon/Blueprints/Actors/CINEMATICS/BP_Fireworkd.NS_Firework_Complex` _array_element_2) true))
  (bind _outactor (`LevelSequencePlayer.CreateLevelSequencePlayer` "/Game/FarmingDungeon/Blueprints/Manager/Cinematic_Montage.Cinematic_Montage"))
  (`MovieSceneSequencePlayer.Play` (`LevelSequenceActor.SequencePlayer` _outactor))
  (bind _returnvalue_2 (`GameplayStatics.SpawnSound2D` "/Game/FarmingDungeon/Audio/Music/Painted_Dreams_Mock-Up.Painted_Dreams_Mock-Up" 1.0 1.0 0.0 null))
  (set `self.OST` _returnvalue_2)
  (`GameplayStatics.PlaySound2D` "/Game/FarmingDungeon/Audio/SE/Fireworks_Grand_Finale_Sound_Effect__FREE_TO_USE_.Fireworks_Grand_Finale_Sound_Effect__FREE_TO_USE_" 0.1 1.0 0.0 null null)
  (`KismetSystemLibrary.Delay` 13.0)
  (bind _returnvalue_3 (`|CreateWidget` "/Game/FarmingDungeon/Blueprints/Widgets/WBP_EndCredits.WBP_EndCredits_C"))
  (`UserWidget.AddToViewport` _returnvalue_3 0))

(fn `IsInteractible`
  (returns (Interactable :type Boolean))
  (return true))

(fn `Tuto`
  (bind _bpc_tutorialmanager (`/Game/FarmingDungeon/Blueprints/Quest/Tutorial/BP_TutorialManager.BPC_TutorialManager` (`self.TutoManagerRef`)))
  (bind _asbp_player (cast `/Game/FarmingDungeon/Blueprints/Characters/BP_Player` (`GameplayStatics.GetPlayerPawn` 0)))
  (if (and (`/Game/FarmingDungeon/Blueprints/Quest/Tutorial/BPC_TutorialManager.HasEnterFarm` (`/Game/FarmingDungeon/Blueprints/Quest/Tutorial/BP_TutorialManager.BPC_TutorialManager` (`self.TutoManagerRef`))) (not (`/Game/FarmingDungeon/Blueprints/Quest/Tutorial/BPC_TutorialManager.StartFight` (`/Game/FarmingDungeon/Blueprints/Quest/Tutorial/BP_TutorialManager.BPC_TutorialManager` (`self.TutoManagerRef`)))))
    (set `/Game/FarmingDungeon/Blueprints/Quest/Tutorial/BPC_TutorialManager.StartFight` true (`/Game/FarmingDungeon/Blueprints/Quest/Tutorial/BP_TutorialManager.BPC_TutorialManager` (`self.TutoManagerRef`)))
    (`/Game/FarmingDungeon/Blueprints/Quest/Tutorial/BPC_TutorialManager.UpdateState` (`/Game/FarmingDungeon/Blueprints/Quest/Tutorial/BP_TutorialManager.BPC_TutorialManager` (`self.TutoManagerRef`)) _asbp_player :!label _label)
    (elif (`/Game/FarmingDungeon/Blueprints/Quest/Tutorial/BPC_TutorialManager.HasFinishFight` _bpc_tutorialmanager)
      (goto _label)
      (elif (`/Game/FarmingDungeon/Blueprints/Quest/Tutorial/BPC_TutorialManager.HasStockedObject` _bpc_tutorialmanager)
        (set `/Game/FarmingDungeon/Blueprints/Quest/Tutorial/BPC_TutorialManager.HasFinishedTalkingToIsabelle` true _bpc_tutorialmanager)
        (goto _label)))))

(fn `UserConstructionScript`
  (`parent.UserConstructionScript`))