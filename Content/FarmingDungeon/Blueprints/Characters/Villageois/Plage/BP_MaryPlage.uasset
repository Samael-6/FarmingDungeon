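; Beach-level villager Blueprint for Mary, an always-interactible NPC with dialogue and quest state.
; It syncs her condition and quest flags with the GameInstance through BPCDialogue, re-reading the condition every Tick.
; The quest-start check simply resets dialogue to the first row, and BeginPlay only calls the parent.
; Disconnected leftover logic holds services widget creation, saved-state loading and quest-based dialogue row selection.
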(event `self.ReceiveBeginPlay`
  (`parent.ReceiveBeginPlay`))

(event `self.UpdateVillagerCondition`
  (params (ResetValue :type Boolean))
  (bind _output_get (set `/Game/FarmingDungeon/Blueprints/Manager/BP_GameInstance.MaryCondition` ResetValue (`/Game/FarmingDungeon/Blueprints/Components/BPC_Dialogue.GameInstanceRef` (`self.BPC_Dialogue`))))
  (bind _output_get_2 (set `self.VillagerCondition` _output_get :!label _label)))

(event `self.ReceiveTick`
  (params (DeltaSeconds :type "Float (single-precision)"))
  (goto _label))

(event `self.UpdateStartedQuest`
  (params (Value :type Boolean))
  (bind _output_get (set `self.HasStartedQuest` Value))
  (set `/Game/FarmingDungeon/Blueprints/Manager/BP_GameInstance.HasStartedMary` _output_get (`/Game/FarmingDungeon/Blueprints/Components/BPC_Dialogue.GameInstanceRef` (`self.BPC_Dialogue`))))

(event `self.UpdateFinishedQuest`
  (set `self.HasFinishedQuest` (`/Game/FarmingDungeon/Blueprints/Manager/BP_GameInstance.HasFinishedMaryQuest` (`/Game/FarmingDungeon/Blueprints/Components/BPC_Dialogue.GameInstanceRef` (`self.BPC_Dialogue`)))))

(event `self.CheckIfQuestSTarted`
  (set `/Game/FarmingDungeon/Blueprints/Components/BPC_Dialogue.CurrentRowNumber` 0 (`self.BPC_Dialogue`)))

(fn `IsInteractible`
  (returns (Interactable :type Boolean))
  (return true))

(fn `UserConstructionScript`
  (`parent.UserConstructionScript`))