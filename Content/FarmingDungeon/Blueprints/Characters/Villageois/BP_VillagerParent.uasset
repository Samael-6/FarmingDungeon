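; Base villager NPC for the village, providing interactable dialogue, quest hooks and scripted walking.
; Interaction opens the dialogue widget and switches to menu input; BPCDialogue supplies rows and advances them by choice until game input is restored.
; When triggered, it follows successive splines on Tick, notifying the tutorial manager at each end.
; Empty quest/condition events serve as override points, and a helper maps dialogue rows to village camera views.
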(event `self.ReceiveBeginPlay`
  (bind _asbp_gm_village (cast `/Game/FarmingDungeon/Blueprints/Manager/GameModes/BP_GM_Village` (`GameplayStatics.GetGameMode`)))
  (set `self.As BP GM Village` _asbp_gm_village)
  (bind _returnvalue (`|CreateWidget` "/Game/FarmingDungeon/Blueprints/Widgets/WBP_DialogueUI.WBP_DialogueUI_C"))
  (bind _output_get (set `self.DialogueHUDRef` _returnvalue))
  (set `/Game/FarmingDungeon/Blueprints/Widgets/WBP_DialogueUI.VillageoisRef` self _output_get)
  (bind _asbp_game_instance (cast `/Game/FarmingDungeon/Blueprints/Manager/BP_GameInstance` (`GameplayStatics.GetGameInstance`)))
  (set `self.As BP Game Instance` _asbp_game_instance)
  (set `/Game/FarmingDungeon/Blueprints/Components/BPC_Dialogue.GameInstanceRef` _asbp_game_instance (`self.BPC_Dialogue`))
  (set `/Game/FarmingDungeon/Blueprints/Components/BPC_Dialogue.VillagerParentRef` self (`self.BPC_Dialogue`))
  (set `self.Text` (`KismetTextLibrary.Conv_StringToText` (`KismetSystemLibrary.GetDisplayName` self))))

(event `self.ReceiveTick`
  (params (DeltaSeconds :type "Float (single-precision)"))
  (if (`self.IsMoving`)
    (`self.MoveAlongSpline` DeltaSeconds)))

(event `Activate`
  (`self.CheckIfQuestSTarted`)
  (`UserWidget.AddToPlayerScreen` (`self.DialogueHUDRef`) 0)
  (`/Game/FarmingDungeon/Blueprints/Components/BPC_Dialogue.GetCurrentDialogueRow` (`self.BPC_Dialogue`))
  (bind _charactername (`/Game/FarmingDungeon/Blueprints/Components/BPC_Dialogue.GetCharacterFromCurrentRow` (`self.BPC_Dialogue`)))
  (bind (_choicestext _dialoguetext) (`/Game/FarmingDungeon/Blueprints/Components/BPC_Dialogue.GetDialogueTextFromCurrentRow` (`self.BPC_Dialogue`)))
  (`/Game/FarmingDungeon/Blueprints/Widgets/WBP_DialogueUI.UpdateDialogueText` (`self.DialogueHUDRef`) _charactername _dialoguetext _choicestext))

(event `Update`
  (params (IndexOfChoice :type Integer))
  (bind _isfinished (`/Game/FarmingDungeon/Blueprints/Components/BPC_Dialogue.IsDialogueFinished` (`self.BPC_Dialogue`) IndexOfChoice))
  (if _isfinished
    (`self.Deactivate`)
    (else
      (`/Game/FarmingDungeon/Blueprints/Components/BPC_Dialogue.ReadNextRow` (`self.BPC_Dialogue`) IndexOfChoice)
      (bind _charactername (`/Game/FarmingDungeon/Blueprints/Components/BPC_Dialogue.GetCharacterFromCurrentRow` (`self.BPC_Dialogue`)))
      (bind (_choicestext _dialoguetext) (`/Game/FarmingDungeon/Blueprints/Components/BPC_Dialogue.GetDialogueTextFromCurrentRow` (`self.BPC_Dialogue`)))
      (`/Game/FarmingDungeon/Blueprints/Widgets/WBP_DialogueUI.UpdateDialogueText` (`self.DialogueHUDRef`) _charactername _dialoguetext _choicestext)
      (`self.UpdateVillagerCondition` false))))

(event `Deactivate`
  (bind _returnvalue (`GameplayStatics.GetPlayerController` 0))
  (bind _returnvalue_2 (pcsubsystem `EnhancedInputLocalPlayerSubsystem` (`GameplayStatics.GetPlayerController` 0)))
  (`Widget.RemoveFromParent` (`self.DialogueHUDRef`))
  (`EnhancedInputSubsystemInterface.ClearAllMappings` _returnvalue_2)
  (message `EnhancedInputSubsystemInterface.AddMappingContext` _returnvalue_2 "/Game/FarmingDungeon/Blueprints/Manager/Inputs/InputActions/IMC_Game.IMC_Game" 0 (struct))
  (`WidgetBlueprintLibrary.SetInputMode_GameOnly` _returnvalue)
  (set `PlayerController.bShowMouseCursor` false _returnvalue)
  (`/Game/FarmingDungeon/Blueprints/Widgets/WBP_DialogueUI.ClearDialogueText` (`self.DialogueHUDRef`))
  (`/Game/FarmingDungeon/Blueprints/Widgets/WBP_PlayerHUD.UpdateQuestBar` (`/Game/FarmingDungeon/Blueprints/Characters/BP_Player.PlayerHUDRef` (`/Game/FarmingDungeon/Blueprints/Manager/BP_GameInstance.Bp_PlayerRef` (`self.As BP Game Instance`)))))

(event `/Game/FarmingDungeon/Blueprints/Interfaces/BPI_Interact.OnInteract`
  (params (Player :type "/Game/FarmingDungeon/Blueprints/Characters/BP_Player Object Reference"))
  (bind _returnvalue (pcsubsystem `EnhancedInputLocalPlayerSubsystem` (`GameplayStatics.GetPlayerController` 0)))
  ;[1 1 1] Comment
  (`self.Activate`)
  (`EnhancedInputSubsystemInterface.ClearAllMappings` _returnvalue)
  (message `EnhancedInputSubsystemInterface.AddMappingContext` _returnvalue "/Game/FarmingDungeon/Blueprints/Manager/Inputs/InputActions/IMC_Menu.IMC_Menu" 0 (struct))
  (set `PlayerController.bShowMouseCursor` true (`GameplayStatics.GetPlayerController` 0)))

(event `UpdateVillagerCondition`
  (params (ResetValue :type Boolean)))

(event `TriggerMovement`
  (set `self.IsMoving` true))

(event `UpdateStartedQuest`
  (params (Value :type Boolean)))

(event `UpdateFinishedQuest`)

(event `CheckIfQuestStarted`)

(fn `ChangeCamViewByIndex`
  (params (RowIndex :type Integer))
  (returns (Enabled :type Boolean))
  (bind (_value _returnvalue) (`BlueprintMapLibrary.Map_Find` (`self.MapsOfCamView`) RowIndex))
  (if _returnvalue
    (if (== (`/Game/FarmingDungeon/Blueprints/Components/BPC_Dialogue.CurrentRowNumber` (`self.BPC_Dialogue`)) RowIndex)
      (if (not (== (`/Game/FarmingDungeon/Blueprints/Manager/GameModes/BP_GM_Village.CameraPlanVillage` (`self.As BP GM Village`)) (`Controller.GetViewTarget` (`GameplayStatics.GetPlayerController` 0))))
        (`/Game/FarmingDungeon/Blueprints/Manager/GameModes/BP_GM_Village.TransitionToCameraPlanVillage` (`self.As BP GM Village`) _value)
        (`self.DisplayAssetsInWorld`)
        (return true)
        (else
          (`/Game/FarmingDungeon/Blueprints/Manager/GameModes/BP_GM_Village.TransitionToCameraPlayer` (`self.As BP GM Village`)))))
    (else
      (return false))))

(fn `IsInteractible`
  (returns (Interactable :type Boolean))
  (return true))

(fn `MoveAlongSpline`
  (params (`Delta Seconds` :type "Float (double-precision)"))
  (bind (_returnvalue_x _returnvalue_y _returnvalue_z) (`KismetMathLibrary.BreakVector` (`SceneComponent.K2_GetComponentLocation` (`self.CapsuleComponent`))))
  (bind _bpc_tutorialmanager (`/Game/FarmingDungeon/Blueprints/Quest/Tutorial/BP_TutorialManager.BPC_TutorialManager` (`self.TutoManagerRef`)))
  (bind _returnvalue (`SplineComponent.GetTransformAtDistanceAlongSpline` (`/Game/FarmingDungeon/Blueprints/Quest/BP_SplineForVillagerMovement.Spline` (`|GetArrayItem` (`self.ListOfSplines`) (`self.IndexOfSpline`))) (`self.DistanceAlongSpline`) "World" false))
  (set `self.Speed` (`MovementComponent.GetMaxSpeed` (`self.CharacterMovement`)))
  (set `self.DistanceAlongSpline` (+ (* `Delta Seconds` 300.0) (`self.DistanceAlongSpline`)))
  (`SceneComponent.K2_SetWorldTransform` (`self.CapsuleComponent`) (`KismetMathLibrary.MakeTransform` (`KismetMathLibrary.MakeVector` (.x (.location _returnvalue)) (.y (.location _returnvalue)) _returnvalue_z) (`KismetMathLibrary.MakeRotator` (.roll (.rotation _returnvalue)) (.pitch (.rotation _returnvalue)) (.yaw (.rotation _returnvalue))) (`SceneComponent.RelativeScale3D` (`self.CapsuleComponent`))) false false)
  (if (> (`self.DistanceAlongSpline`) (`SplineComponent.GetSplineLength` (`/Game/FarmingDungeon/Blueprints/Quest/BP_SplineForVillagerMovement.Spline` (`|GetArrayItem` (`self.ListOfSplines`) (`self.IndexOfSpline`)))))
    (set `self.IsMoving` false)
    (set `self.DistanceAlongSpline` 0.0)
    (set `self.IndexOfSpline` (+ (`self.IndexOfSpline`) 1))
    (set `self.Speed` 0.0)
    (`/Engine/EditorBlueprintResources/StandardMacros.IsValid` _bpc_tutorialmanager
      (:`Is Valid`
        (`/Game/FarmingDungeon/Blueprints/Quest/Tutorial/BPC_TutorialManager.UpdateDialogueWithEvent` _bpc_tutorialmanager)))))

(fn `UpdateRowNumberByQuest`
  (params (NewParam :type Integer))
  (set `/Game/FarmingDungeon/Blueprints/Components/BPC_Dialogue.CurrentRowNumber` NewParam (`self.BPC_Dialogue`)))

(fn `UserConstructionScript`)