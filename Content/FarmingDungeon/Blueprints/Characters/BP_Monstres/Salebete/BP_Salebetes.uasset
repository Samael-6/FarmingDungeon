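; Salebete monster Blueprint for FarmingDungeon, a ranged enemy child that sets its stats and loot on BeginPlay through parent logic.
; Each Tick it turns toward the player and runs player detection, flagging IsRMove when none is detected; the Tick attack branch is hard-wired off.
; AnimAttacked spawns a projectile fired at the player's position with a height offset.
; AnimGetHit briefly swaps the mesh to a damage material.
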(event `self.ReceiveBeginPlay`
  (`parent.ReceiveBeginPlay`)
  (bind _asbp_game_instance (cast `/Game/FarmingDungeon/Blueprints/Manager/BP_GameInstance` (`GameplayStatics.GetGameInstance`)))
  (bind _asbp_player (cast `/Game/FarmingDungeon/Blueprints/Characters/BP_Player` (`GameplayStatics.GetPlayerPawn` 0)))
  (`self.SetVariables` 3.0 0.5 1.0 0.0 400.0 _asbp_game_instance _asbp_player null "/Game/FarmingDungeon/Blueprints/Actors/BP_Monstres/LootMonstres/BP_LootSalbete.BP_LootSalbete_C" "NewEnumerator10"))

(event `self.ReceiveTick`
  (params (DeltaSeconds :type "Float (single-precision)"))
  (`parent.ReceiveTick` DeltaSeconds)
  (`self.K2_SetActorRotation` (`KismetMathLibrary.FindLookAtRotation` (`SceneComponent.K2_GetComponentLocation` (`self.Mesh`)) (`SceneComponent.K2_GetComponentLocation` (`Character.Mesh` (`self.Ref_BP_Player`)))))
  (`self.DetectionPlayer` (`self.Cube`))
  (if false
    (`KismetSystemLibrary.Delay` 2.0)
    (`/Game/FarmingDungeon/Blueprints/Interfaces/BPI_AnimAttack.AnimAttacked`)
    (elif (not (`self.IsPlayerDetected`))
      (set `self.IsRMove` true))))

(event `self.AnimGetHit`
  (bind _mesh (`self.Mesh`))
  ;[1 1 1] Animation lorsque le monstre reçoit un coup
  (`PrimitiveComponent.SetMaterial` _mesh 0 "/Game/FarmingDungeon/Model3D/Monstres/M_DamagedTest.M_DamagedTest")
  (`KismetSystemLibrary.Delay` 0.2)
  (`PrimitiveComponent.SetMaterial` _mesh 0 (`self.M_Monster`)))

(event `self.AnimAttacked`
  (bind (_returnvalue_location _returnvalue_rotation _returnvalue_scale) (`KismetMathLibrary.BreakTransform` (`self.GetTransform`)))
  (bind (_returnvalue_x _returnvalue_y _returnvalue_z) (`KismetMathLibrary.BreakVector` (`SceneComponent.K2_GetComponentLocation` (`Character.Mesh` (`self.Ref_BP_Player`)))))
  (bind _returnvalue (`|SpawnActorFromClass` (`self.Projectile`) (`KismetMathLibrary.MakeTransform` _returnvalue_location _returnvalue_rotation _returnvalue_scale) "AlwaysSpawn" "MultiplyWithRoot" null null))
  (`/Engine/EditorBlueprintResources/StandardMacros.IsValid` _returnvalue
    (:`Is Valid`
      (`/Game/FarmingDungeon/Blueprints/Actors/BP_Monstres/BP_TireSabeltte.Shoot` _returnvalue (`KismetMathLibrary.MakeVector` _returnvalue_x _returnvalue_y (+ _returnvalue_z 50.0)) (`self.Attack_Monstre`) 300.0 (`self.Ref_BP_GameInstance`) (`self.Ref_BP_Player`)))
    (:`Is Not Valid`
      (`KismetSystemLibrary.PrintString` "Hello"))))

(fn `UserConstructionScript`
  (`parent.UserConstructionScript`))