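; BP_FrongusBig is a monster character, the big Frongus, built on a parent monster class.
; BeginPlay passes its stats, loot and player/GameInstance references to the parent's SetVariables and applies its movement speed.
; Attack is DoOnce-gated: after a wind-up delay, a short forward sphere trace damages the player through BPC_PV, then a cooldown resets it.
; AnimGetHit briefly swaps in a damage material as hit feedback.
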(event `self.ReceiveBeginPlay`
  (`parent.ReceiveBeginPlay`)
  (bind _asbp_game_instance (cast `/Game/FarmingDungeon/Blueprints/Manager/BP_GameInstance` (`GameplayStatics.GetGameInstance`)))
  (bind _asbp_player (cast `/Game/FarmingDungeon/Blueprints/Characters/BP_Player` (`GameplayStatics.GetPlayerPawn` 0)))
  (`self.SetVariables` 10.0 100.0 400.0 6.0 1.0 100.0 _asbp_game_instance _asbp_player self "/Game/FarmingDungeon/Blueprints/Actors/BP_Monstres/LootMonstres/BP_LootFrongus.BP_LootFrongus_C" "NewEnumerator9" 2)
  (set `CharacterMovementComponent.MaxWalkSpeed` (`self.MSpeed`) (`self.CharacterMovement`)))

(event `self.Attack`
  (bind _returnvalue (`self.K2_GetActorLocation`))
  (bind _ref_bp_gameinstance (`self.Ref_BP_GameInstance`))
  (`/Engine/EditorBlueprintResources/StandardMacros.DoOnce` false :!label _label
    (:`Completed`
      (`KismetSystemLibrary.Delay` 0.7)
      (bind _outhit (`KismetSystemLibrary.SphereTraceSingle` _returnvalue (+ _returnvalue (* (`self.GetActorForwardVector`) 100.0)) 50.0 "TraceTypeQuery1"))
      (bind (_bblockinghit _binitialoverlap _time _distance _location _impactpoint _normal _impactnormal _physmat _hitactor) (`GameplayStatics.BreakHitResult` _outhit))
      (if (== _hitactor (`self.Ref_BP_Player`))
        (bind _returnvalue_2 (`self.GetComponentByClass` _hitactor "/Game/FarmingDungeon/Blueprints/Components/BPC_PV.BPC_PV_C"))
        (`/Game/FarmingDungeon/Blueprints/Components/BPC_PV.Get_Hit` _returnvalue_2 (`self.Attack_Monstre`))
        (`/Game/FarmingDungeon/Blueprints/Components/BPC_PV.Update_PVPlayer` _returnvalue_2 _ref_bp_gameinstance)
        (`KismetSystemLibrary.PrintString` (`KismetStringLibrary.Conv_DoubleToString` (`/Game/FarmingDungeon/Blueprints/Manager/BP_GameInstance.PV_Player` _ref_bp_gameinstance))))
      (`KismetSystemLibrary.Delay` 1.0)
      (goto _label :!via `Reset`))))

(event `self.ReceiveTick`
  (params (DeltaSeconds :type "Float (single-precision)"))
  (`parent.ReceiveTick` DeltaSeconds))

(event `self.AnimGetHit`
  (bind _mesh (`self.Mesh`))
  ;[1 1 1] Animation lorsque le monstre reçoit un coup
  (`PrimitiveComponent.SetMaterial` _mesh 0 "/Game/FarmingDungeon/Model3D/Monstres/M_DamagedTest.M_DamagedTest")
  (`KismetSystemLibrary.Delay` 0.2)
  (`PrimitiveComponent.SetMaterial` _mesh 0 (`self.M_Monster`)))

(fn `UserConstructionScript`
  (`parent.UserConstructionScript`))