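; BP_Sabelttes is a roaming ranged monster Blueprint that detects the player and attacks with projectiles.
; BeginPlay passes its stats, game instance, player and loot class to inherited setup, then starts random movement.
; Tick runs player detection and, while attacking, spawns a projectile every frame from the sphere's relative transform, aimed at the player's mesh.
; A hit briefly swaps the sphere to a damage material.
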(event `self.ReceiveBeginPlay`
  (`parent.ReceiveBeginPlay`)
  (bind _asbp_game_instance (cast `/Game/FarmingDungeon/Blueprints/Manager/BP_GameInstance` (`GameplayStatics.GetGameInstance`)))
  (bind _asbp_player (cast `/Game/FarmingDungeon/Blueprints/Characters/BP_Player` (`GameplayStatics.GetPlayerPawn` 0)))
  (`self.SetVariables` 0.5 3.0 500.0 0.0 _asbp_game_instance _asbp_player "/Game/FarmingDungeon/Blueprints/Actors/BP_Monstres/BP_LootMonstreParent.BP_LootMonstreParent_C")
  (`self.RandomMove` self))

(event `self.ReceiveTick`
  (params (DeltaSeconds :type "Float (single-precision)"))
  (`parent.ReceiveTick` DeltaSeconds)
  (`self.DetectionPlayer` (`self.Sphere`))
  (if (`self.IsAttacking`)
    (`/Game/FarmingDungeon/Blueprints/Interfaces/BPI_AnimAttack.AnimAttacked`)))

(event `self.AnimGetHit`
  (bind _sphere (`self.Sphere`))
  ;[1 1 1] Animation lorsque le monstre reçoit un coup
  (`PrimitiveComponent.SetMaterial` _sphere 0 "/Game/FarmingDungeon/Model3D/Monstres/M_DamagedTest.M_DamagedTest")
  (`KismetSystemLibrary.Delay` 0.2)
  (`PrimitiveComponent.SetMaterial` _sphere 0 (`self.M_Monster`)))

(event `self.AnimAttacked`
  (bind (_returnvalue_location _returnvalue_rotation _returnvalue_scale) (`KismetMathLibrary.BreakTransform` (`SceneComponent.GetRelativeTransform` (`self.Sphere`))))
  (bind _returnvalue (`|SpawnActorFromClass` (`self.Projectile`) (`KismetMathLibrary.MakeTransform` (+ _returnvalue_location 10.0) _returnvalue_rotation _returnvalue_scale) "AlwaysSpawn" "MultiplyWithRoot" null null))
  (`/Game/FarmingDungeon/Blueprints/Actors/BP_Monstres/BP_TireSabeltte.Shoot` _returnvalue (`SceneComponent.K2_GetComponentLocation` (`Character.Mesh` (`self.Ref_BP_Player`))) (`self.Attack_Monstre`) (`self.Ref_BP_GameInstance`)))

(fn `UserConstructionScript`
  (`parent.UserConstructionScript`))