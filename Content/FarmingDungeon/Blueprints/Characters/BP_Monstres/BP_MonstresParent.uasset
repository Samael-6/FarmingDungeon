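; Parent Blueprint for farming-dungeon monsters that wander, chase the player and drop loot on death.
; RandomMove picks random points around world X/Y origin at spawn height, repeating until the player is detected, then ChasePlayer follows until in attack range.
; Both movements use VInterpTo on timelines sized by distance over speed.
; DetectionPlayer sets range flags, SetVariables receives stats, and BPCPV's death event spawns Loot and destroys the actor.
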(event `self.ReceiveBeginPlay`
  (bind (_returnvalue_x _returnvalue_y _returnvalue_z) (`KismetMathLibrary.BreakVector` (`self.K2_GetActorLocation`)))
  (bind _asbp_game_instance (cast `/Game/FarmingDungeon/Blueprints/Manager/BP_GameInstance` (`GameplayStatics.GetGameInstance`)))
  (set `self.Ref_BP_GameInstance` _asbp_game_instance)
  (bind _asbp_player (cast `/Game/FarmingDungeon/Blueprints/Characters/BP_Player` (`GameplayStatics.GetPlayerPawn` 0)))
  (set `self.Ref_BP_Player` _asbp_player)
  (add `/Game/FarmingDungeon/Blueprints/Components/BPC_PV.ED_Mort` (`self.BPC_PV`) (delegate `OnMonsterDead`))
  (set `self.InitilPosition` (`KismetMathLibrary.MakeVector` 0.0 0.0 _returnvalue_z)))

(event `OnMonsterDead`
  (`|SpawnActorFromClass` (`self.Loot`) (`self.GetTransform`) "Undefined" "MultiplyWithRoot" null null)
  (`KismetSystemLibrary.PrintString` "XP ARME")
  (clear `/Game/FarmingDungeon/Blueprints/Components/BPC_PV.ED_Mort` (`self.BPC_PV`))
  (`self.K2_DestroyActor`))

(event `self.ReceiveTick`
  (params (DeltaSeconds :type "Float (single-precision)")))

(event `RandomMove`
  (params (BP_Monstre :type "/Game/FarmingDungeon/Blueprints/Characters/BP_Monstres/BP_MonstresParent Object Reference"))
  (bind (_returnvalue_x _returnvalue_y) (`KismetMathLibrary.BreakVector` (`self.K2_GetActorLocation`)))
  (bind (_returnvalue_x_2 _returnvalue_y_2) (`KismetMathLibrary.BreakVector` (`KismetMathLibrary.RandomUnitVector`)))
  (bind (_mtargetlocationtest_x _mtargetlocationtest_y) (`KismetMathLibrary.BreakVector` (`self.MTargetLocationTest`)))
  (bind _mradius (`self.MRadius`))
  ;[1 1 1] Déplacement random des monstres
  (set `self.MTargetLocationTest` (+ (`self.InitilPosition`) (`KismetMathLibrary.MakeVector` (* _returnvalue_x_2 _mradius) (* _returnvalue_y_2 _mradius))))
  (bind _time (`self.CalculateTimeFromDistance` _mtargetlocationtest_x _mtargetlocationtest_y _returnvalue_x _returnvalue_y))
  (`TimelineComponent.SetTimelineLength` (`self.Timeline`) (* _time 2.0))
  (bind (_direction _alpha) (`Timeline|Timeline` :!via `PlayFromStart`)
    (:`Update`
      (`self.K2_SetActorLocation` (`KismetMathLibrary.VInterpTo` (`self.K2_GetActorLocation`) (`self.MTargetLocationTest`) _alpha (`self.MSpeed`)) true))
    (:`Finished`
      (`KismetSystemLibrary.Delay` 0.1)
      (if (`self.IsPlayerDetected`)
        (`KismetSystemLibrary.PrintString` "TROUVE" true true (struct :`R` 1.0 :`B` 0.874392 :`A` 1.0))
        (set `self.IsRMove` false)
        (`self.ChasePlayer`)
        (else
          (`self.RandomMove` null))))))

(event `ChasePlayer`
  (bind (_returnvalue_x _returnvalue_y) (`KismetMathLibrary.BreakVector` (`self.K2_GetActorLocation`)))
  (bind (_returnvalue_x_2 _returnvalue_y_2) (`KismetMathLibrary.BreakVector` (`self.K2_GetActorLocation` (`self.Ref_BP_Player`))))
  (bind _time (`self.CalculateTimeFromDistance` _returnvalue_x_2 _returnvalue_y_2 _returnvalue_x _returnvalue_y))
  (`TimelineComponent.SetTimelineLength` (`self.ChasedPlayer`) _time)
  (bind (_direction _alpha) (`Timeline|ChasedPlayer` :!via `PlayFromStart` :!label _label)
    (:`Update`
      (if (`self.IsAttacking`)
        (goto _label :!via `Stop`)
        (else
          (`self.K2_SetActorLocation` (`KismetMathLibrary.VInterpTo` (`self.K2_GetActorLocation`) (`self.K2_GetActorLocation` (`self.Ref_BP_Player`)) _alpha (`self.MSpeed`))))))))

(fn `CalculateTimeFromDistance`
  (params (Xa :type "Float (double-precision)") (Ya :type "Float (double-precision)") (Xb :type "Float (double-precision)") (Yb :type "Float (double-precision)"))
  (returns (Time :type "Float (double-precision)"))
  (return (/ (`KismetMathLibrary.Abs` (`KismetMathLibrary.Sqrt` (+ (`KismetMathLibrary.Square` (- Xa Xb)) (`KismetMathLibrary.Square` (- Ya Yb))))) (`self.MSpeed`))))

(fn `DetectionPlayer`
  (params (StaticMesh :type "SceneComponent Object Reference"))
  (bind (_returnvalue_x _returnvalue_y _returnvalue_z) (`KismetMathLibrary.BreakVector` (`SceneComponent.K2_GetComponentLocation` StaticMesh)))
  (bind (_returnvalue_x_2 _returnvalue_y_2 _returnvalue_z_2) (`KismetMathLibrary.BreakVector` (`SceneComponent.K2_GetComponentLocation` (`Character.Mesh` (`self.Ref_BP_Player`)))))
  (bind _returnvalue (- _returnvalue_x_2 _returnvalue_x))
  (bind _returnvalue_2 (- _returnvalue_y_2 _returnvalue_y))
  (bind _returnvalue_3 (- _returnvalue_z_2 _returnvalue_z))
  (bind _returnvalue_4 (`KismetMathLibrary.Sqrt` (+ (* _returnvalue _returnvalue) (* _returnvalue_2 _returnvalue_2) (* _returnvalue_3 _returnvalue_3))))
  (set `self.IsPlayerDetected` (<= _returnvalue_4 (`self.RadiusDetectionPlayer`)))
  (set `self.IsAttacking` (<= _returnvalue_4 (`self.RadiusAttackPlayer`))))

(fn `SetVariables`
  (params (Attack :type "Float (double-precision)") (PV :type "Float (double-precision)") (RadiusDetectPlayer :type "Float (double-precision)") (RadiusAttackPlayer :type "Float (double-precision)") (GameInstance :type "/Game/FarmingDungeon/Blueprints/Manager/BP_GameInstance Object Reference") (Player :type "/Game/FarmingDungeon/Blueprints/Characters/BP_Player Object Reference") (Loot :type "/Game/FarmingDungeon/Blueprints/Actors/BP_LootParent Class Reference"))
  (set `self.Attack_Monstre` Attack)
  (set `/Game/FarmingDungeon/Blueprints/Components/BPC_PV.PV` PV (`self.BPC_PV`))
  (set `self.RadiusDetectionPlayer` RadiusDetectPlayer)
  (set `self.RadiusAttackPlayer` RadiusAttackPlayer)
  (set `self.Ref_BP_GameInstance` GameInstance)
  (set `self.Ref_BP_Player` Player)
  (set `self.Loot` Loot))

(fn `Spawn Loot`
  (switch `int` 0
    (:`0`
      (set `self.ListeMonstre` (`/Game/FarmingDungeon/Blueprints/Manager/BP_GameInstance.ListeMonstresF` (`self.Ref_BP_GameInstance`))))
    (:`1`
      (set `self.ListeMonstre` (`/Game/FarmingDungeon/Blueprints/Manager/BP_GameInstance.ListeMonstresM` (`self.Ref_BP_GameInstance`)))))
  (for (_array_element _array_index) (`self.ListeMonstre`)
    (if (== _array_element (`GameplayStatics.GetObjectClass` self))
      (set `self.IndexLoot` _array_index)
      (break)))
  (`|SpawnActorFromClass` (`|GetArrayItem` (`/Game/FarmingDungeon/Blueprints/Manager/BP_GameInstance.ListeLootMonstresF` (`self.Ref_BP_GameInstance`)) (`self.IndexLoot`)) (`self.GetTransform`) "Undefined" "MultiplyWithRoot" null null))

(fn `UserConstructionScript`)