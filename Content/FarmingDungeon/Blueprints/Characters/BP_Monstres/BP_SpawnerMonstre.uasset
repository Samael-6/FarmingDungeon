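; Monster spawner actor for the dungeon that spawns its Monstre class at its own transform when play begins.
; BeginPlay caches the game instance and calls SpawnMonster, which spawns only while IsActive, always spawning with collision adjustment, then clears the flag.
; MonsterChoice is an empty stub with disconnected logic for difficulty-weighted random selection meant to scale with dungeon level.
; GetMonsterFromList returns a list entry by index.
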(event `self.ReceiveBeginPlay`
  (bind _asbp_game_instance (cast `/Game/FarmingDungeon/Blueprints/Manager/BP_GameInstance` (`GameplayStatics.GetGameInstance`)))
  (set `self.BP_GameInstance_Ref` _asbp_game_instance)
  (`self.SpawnMonster`))

(event `self.ReceiveTick`
  (params (DeltaSeconds :type "Float (single-precision)")))

(fn `GetMonsterFromList`
  (params (ListeMonster :type "Array of /Game/FarmingDungeon/Blueprints/Characters/BP_Monstres/BP_MonstresParent Class Reference") (Index :type Integer))
  (returns (Monstre :type "/Game/FarmingDungeon/Blueprints/Characters/BP_Monstres/BP_MonstresParent Class Reference"))
  (return (`|GetArrayItem` ListeMonster Index)))

(fn `MonsterChoice`
  (params (ListeMonstre :type "Map of /Game/FarmingDungeon/Blueprints/Characters/BP_Monstres/BP_MonstresParent Class Reference to Integer") (Point :type Integer)))

(fn `SpawnMonster`
  (if (`self.IsActive`)
    (`|SpawnActorFromClass` (`self.Monstre`) (`self.GetTransform` self) "AdjustIfPossibleButAlwaysSpawn" "MultiplyWithRoot" null null)
    (set `self.IsActive` false)))

(fn `UserConstructionScript`)