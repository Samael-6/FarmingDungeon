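; BP_Fongus is a monster that configures an inherited monster base with its attack, hit points, loot class and references to the game instance and player.
; BeginPlay applies these stats after calling the parent.
; The construction script also sets detection and attack radii, but its player cast has no input, so that setup never completes.
; AnimGetHit briefly swaps the sphere's material to flash damage.
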(event `self.ReceiveBeginPlay`
  (`parent.ReceiveBeginPlay`)
  (bind _asbp_game_instance (cast `/Game/FarmingDungeon/Blueprints/Manager/BP_GameInstance` (`GameplayStatics.GetGameInstance`)))
  (bind _asbp_player (cast `/Game/FarmingDungeon/Blueprints/Characters/BP_Player` (`GameplayStatics.GetPlayerPawn` 0)))
  (`self.SetVariables` 0.5 5.0 0.0 0.0 _asbp_game_instance _asbp_player "/Game/FarmingDungeon/Blueprints/Actors/BP_Monstres/BP_LootMonstreParent.BP_LootMonstreParent_C"))

(event `self.AnimGetHit`
  (bind _sphere (`self.Sphere`))
  ;[1 1 1] Animation lorsque le monstre reçoit un coup
  (`PrimitiveComponent.SetMaterial` _sphere 0 "/Game/FarmingDungeon/Model3D/Monstres/M_DamagedTest.M_DamagedTest")
  (`KismetSystemLibrary.Delay` 0.2)
  (`PrimitiveComponent.SetMaterial` _sphere 0 (`self.M_Monster`)))

(event `self.ReceiveTick`
  (params (DeltaSeconds :type "Float (single-precision)"))
  (`parent.ReceiveTick` DeltaSeconds))

(fn `UserConstructionScript`
  (`parent.UserConstructionScript`)
  (bind _asbp_game_instance (cast `/Game/FarmingDungeon/Blueprints/Manager/BP_GameInstance` (`GameplayStatics.GetGameInstance`)))
  (bind _asbp_player (cast `/Game/FarmingDungeon/Blueprints/Characters/BP_Player` _))
  (`self.SetVariables` 0.5 5.0 700.0 150.0 _asbp_game_instance _asbp_player "/Game/FarmingDungeon/Blueprints/Actors/BP_Monstres/BP_LootMonstreParent.BP_LootMonstreParent_C"))