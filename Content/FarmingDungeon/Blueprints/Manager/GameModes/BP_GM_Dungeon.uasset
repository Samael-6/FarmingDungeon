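; Dungeon game mode that builds a randomized room sequence for the current dungeon floor stored in the game instance.
; MakeStage brackets the list with rest rooms and has a loop drawing mob or loot rooms, with GetRoom checking picks against the previous room.
; BeginPlay derives per-fight room points from floor depth and fight-room count.
; EnterRoom triggers the spawner manager's resources and monsters, gated by per-room activation flags.
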(event `self.ReceiveBeginPlay`
  (bind _asbp_game_instance (cast `/Game/FarmingDungeon/Blueprints/Manager/BP_GameInstance` (`GameplayStatics.GetGameInstance`)))
  (bind _output_get (set `self.GameInstance` _asbp_game_instance))
  (bind _returnvalue (+ 2 (`/Game/FarmingDungeon/Blueprints/Manager/BP_GameInstance.StageDungeonF` _output_get)))
  (`self.MakeStage` _returnvalue)
  (bind _output_get_2 (set `self.ValueTempFloat` (* (+ (`/Game/FarmingDungeon/Blueprints/Manager/BP_GameInstance.StageDungeonF` _output_get) 0.5) 10.0)))
  (set `self.RoomPoints` (`KismetMathLibrary.FTrunc` (/ (/ _output_get_2 (`KismetMathLibrary.Conv_IntToDouble` _returnvalue)) (`self.NbRoomFight`)))))

(event `EnterRoom`
  (bind _returnvalue (`GameplayStatics.GetActorOfClass` "/Game/FarmingDungeon/Blueprints/Actors/BP_ManagerSpawner.BP_ManagerSpawner_C"))
  (bind _isactivable (`self.CheckSpawnActivation` (`self.CurrentStage`)))
  (if _isactivable
    (`/Game/FarmingDungeon/Blueprints/Actors/BP_ManagerSpawner.SpawnRessources` _returnvalue 0)
    (`/Game/FarmingDungeon/Blueprints/Actors/BP_ManagerSpawner.SpawnMonsters` _returnvalue 0)))

(fn `CheckSpawnActivation`
  (params (RoomIndex :type Integer))
  (returns (IsActivable :type Boolean))
  (bind _isspawnneractivate (`self.IsSpawnnerActivate`))
  (`KismetArrayLibrary.Array_Set` _isspawnneractivate 0 true)
  (return (not (`|GetArrayItem` _isspawnneractivate RoomIndex))))

(fn `GetRoom`
  (params (RoomList :type "Array of Name"))
  (returns (RoomName :type Name) (IsValid :type Boolean))
  (bind _stage (`self.Stage`))
  (bind _output (`|GetArrayItem` RoomList (`KismetMathLibrary.RandomIntegerInRange` 0 (- (`KismetArrayLibrary.Array_Length` RoomList) 1))))
  (return _output (== _output (`|GetArrayItem` _stage (- (`KismetArrayLibrary.Array_Length` _stage) 1)))))

(fn `MakeStage`
  (params (NBSalle :type Integer))
  (bind _stage (`self.Stage`))
  (`KismetArrayLibrary.Array_Clear` _stage)
  (`KismetArrayLibrary.Array_Add` _stage "Lvl_Repos")
  (set `self.ValueTempInt` NBSalle)
  (while (<= (`self.ValueTempInt`) 0)
    (switch `int` (`KismetMathLibrary.RandomIntegerInRange` 0 2)
      (:`Default`
        (bind (_roomname _isvalid) (`self.GetRoom` (`self.ListSalleMob`) :!label _label))
        (if _isvalid
          (`KismetArrayLibrary.Array_Add` (`self.IsSpawnnerActivate`) true)
          (`KismetArrayLibrary.Array_Add` (`self.Stage`) _roomname)
          (`/Engine/EditorBlueprintResources/StandardMacros.IncrementInt` (`self.NbRoomFight`)
            (:`  `
              (set `self.ValueTempInt` (- (`self.ValueTempInt`) 1) :!label _label_2)))))
      (:`0`
        (goto _label))
      (:`1`
        (bind (_roomname_2 _isvalid_2) (`self.GetRoom` (`self.ListSalleLoot`)))
        (if _isvalid_2
          (`KismetArrayLibrary.Array_Add` (`self.IsSpawnnerActivate`) true)
          (`KismetArrayLibrary.Array_Add` (`self.Stage`) _roomname_2)
          (goto _label_2)))))
  (`KismetArrayLibrary.Array_Add` (`self.Stage`) "Lvl_Repos"))

(fn `UserConstructionScript`)