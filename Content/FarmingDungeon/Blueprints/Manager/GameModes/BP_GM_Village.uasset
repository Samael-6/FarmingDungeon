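; Village game mode Blueprint that switches the player's view between a village overview camera and the player pawn.
; On BeginPlay it caches the game instance, the player, a transitions widget and the level's CameraActor found by class.
; Two transition events show the widget, play its fade-to-black animation, wait for it to finish, then change the controller's view target and remove the widget.
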(event `self.ReceiveBeginPlay`
  (bind _asbp_game_instance (cast `/Game/FarmingDungeon/Blueprints/Manager/BP_GameInstance` (`GameplayStatics.GetGameInstance`)))
  (set `self.As BP Game Instance` _asbp_game_instance)
  (bind _asbp_player (cast `/Game/FarmingDungeon/Blueprints/Characters/BP_Player` (`GameplayStatics.GetPlayerPawn` 0)))
  (set `self.As BP Player` _asbp_player)
  (bind _returnvalue (`|CreateWidget` "/Game/FarmingDungeon/Blueprints/Widgets/WBP_Transitions.WBP_Transitions_C"))
  (set `self.WBP_TransitionsRef` _returnvalue)
  (bind _returnvalue_2 (`GameplayStatics.GetActorOfClass` "/Script/Engine.CameraActor"))
  (set `self.CameraPlanVillage` _returnvalue_2))

(event `TransitionToCameraPlanVillage`
  (bind _wbp_transitionsref (`self.WBP_TransitionsRef`))
  (bind _fadeout_black (`/Game/FarmingDungeon/Blueprints/Widgets/WBP_Transitions.FadeOut_Black` _wbp_transitionsref))
  (`UserWidget.AddToViewport` (`self.WBP_TransitionsRef`) 0)
  (`UserWidget.PlayAnimation` _wbp_transitionsref _fadeout_black 0.0 1 "Forward" 1.0 false)
  (`KismetSystemLibrary.Delay` (`WidgetAnimation.GetEndTime` _fadeout_black))
  (`Widget.RemoveFromParent` (`self.WBP_TransitionsRef`))
  (`PlayerController.SetViewTargetWithBlend` (`GameplayStatics.GetPlayerController` 0) (`self.CameraPlanVillage`) 0.0 "VTBlend_Linear" 0.0 false))

(event `TransitionToCameraPlayer`
  (bind _wbp_transitionsref (`self.WBP_TransitionsRef`))
  (bind _fadeout_black (`/Game/FarmingDungeon/Blueprints/Widgets/WBP_Transitions.FadeOut_Black` _wbp_transitionsref))
  (`UserWidget.AddToViewport` (`self.WBP_TransitionsRef`) 0)
  (`UserWidget.PlayAnimation` _wbp_transitionsref _fadeout_black 0.0 1 "Forward" 1.0 false)
  (`KismetSystemLibrary.Delay` (`WidgetAnimation.GetEndTime` _fadeout_black))
  (`PlayerController.SetViewTargetWithBlend` (`GameplayStatics.GetPlayerController` 0) (`self.As BP Player`) 0.0 "VTBlend_Linear" 0.0 false)
  (`Widget.RemoveFromParent` (`self.WBP_TransitionsRef`)))

(fn `UserConstructionScript`)