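; Monster spawner actor for the farming dungeon that picks a monster class by dungeon level and spawns it at its own transform.
; MonsterChoice rolls the first list entry against a medium-monster rate that rises with level, then the second against a reduced small-monster rate, with later entries as fallback.
; SpawnMonster spawns the chosen class only while active, ignoring collisions.
; BeginPlay caches the game instance, which is otherwise unused here.
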(event `self.ReceiveBeginPlay`
  (bind _asbp_game_instance (cast `/Game/FarmingDungeon/Blueprints/Manager/BP_GameInstance` (`GameplayStatics.GetGameInstance`)))
  (set `self.BP_GameInstance_Ref` _asbp_game_instance))

(event `self.ReceiveTick`
  (params (DeltaSeconds :type "Float (single-precision)")))

(fn `GetMonsterFromList`
  (params (ListeMonster :type "Array of /Game/FarmingDungeon/Blueprints/Actors/BP_MonstreParent Class Reference") (Index :type Integer))
  (returns (Monstre :type "/Game/FarmingDungeon/Blueprints/Actors/BP_MonstreParent Class Reference"))
  (return (`|GetArrayItem` ListeMonster Index)))

(fn `MonsterChoice`
  (params (ListeMonstre :type "Array of /Game/FarmingDungeon/Blueprints/Actors/BP_MonstreParent Class Reference") (LvlDungeuon :type Integer))
  (set `self.TauxMonstresMoy` (- (* LvlDungeuon 10) 10))
  (set `self.TauxMonstresPetits` (- (`self.TauxMonstresPetits`) (/ (`self.TauxMonstresMoy`) 2)))
  (for (_array_element _array_index) ListeMonstre
    (switch `int` _array_index
      (:`Default`
        (set `self.Monstre` _array_element))
      (:`0`
        (if (> (`self.TauxMonstresMoy`) (`KismetMathLibrary.RandomIntegerInRange` 0 100))
          (set `self.Monstre` _array_element)
          (break)))
      (:`1`
        (if (> (`self.TauxMonstresPetits`) (`KismetMathLibrary.RandomIntegerInRange` 0 100))
          (set `self.Monstre` _array_element)
          (break))))))

(fn `SpawnMonster`
  (if (`self.IsActive`)
    (`|SpawnActorFromClass` (`self.Monstre`) (`self.GetTransform` self) "AlwaysSpawn" "MultiplyWithRoot" null null)))

(fn `UserConstructionScript`)