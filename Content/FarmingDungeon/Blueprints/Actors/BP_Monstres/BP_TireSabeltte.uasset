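; Monster projectile actor that flies toward a player position captured when Shoot is called, which also stores damage and the game instance.
; While shooting, Tick moves the mesh in a straight line at ShootSpeed, without sweep, and destroys the actor near the target.
; A blocking hit calls GetHit with zero, not the stored Damage, and UpdatePVPlayer on the hit actor's BPC_PV component.
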(event `self.ReceiveTick`
  (params (DeltaSeconds :type "Float (single-precision)"))
  (bind _staticmesh (`self.StaticMesh`))
  (if (`self.IsShooting`)
    (bind _sweephitresult (`SceneComponent.K2_SetWorldLocation` _staticmesh (+ (`SceneComponent.K2_GetComponentLocation` _staticmesh) (* (* DeltaSeconds (`self.ShootSpeed`)) (`KismetMathLibrary.Normal` (- (`self.Target`) (`SceneComponent.K2_GetComponentLocation` (`self.StaticMesh`)))))) false false))
    (bind (_bblockinghit _binitialoverlap _time _distance _location _impactpoint _normal _impactnormal _physmat _hitactor) (`GameplayStatics.BreakHitResult` _sweephitresult))
    (if _bblockinghit
      (bind _returnvalue (`self.GetComponentByClass` _hitactor "/Game/FarmingDungeon/Blueprints/Components/BPC_PV.BPC_PV_C"))
      (`/Game/FarmingDungeon/Blueprints/Components/BPC_PV.Get_Hit` _returnvalue 0.0)
      (`/Game/FarmingDungeon/Blueprints/Components/BPC_PV.Update_PVPlayer` _returnvalue (`self.GameInstance`))
      (elif (== (`SceneComponent.K2_GetComponentLocation` (`self.StaticMesh`)) (`self.Target`) :`ErrorTolerance` 10.0)
        (set `self.IsShooting` false)
        (`self.K2_DestroyActor`)))))

(fn `Shoot`
  (params (PlayerPosition :type "Vector Structure") (Damage :type "Float (double-precision)") (GameInstance :type "/Game/FarmingDungeon/Blueprints/Manager/BP_GameInstance Object Reference"))
  (set `self.Target` PlayerPosition)
  (set `self.Damage` Damage)
  (set `self.GameInstance` GameInstance)
  (set `self.IsShooting` true))

(fn `UserConstructionScript`)