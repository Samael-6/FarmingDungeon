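; BP_Camionette is an interactable van actor that opens the van inventory screen for the player.
; BeginPlay creates WBP_InventaireCamionette and caches BP_GameInstance, which holds the player's item names and counts.
; OnInteract (BPI_Interface) switches input from game to menu mapping, shows the cursor, copies each inventory slot into the widget and displays it.
; The closing branch that restores game input and removes the widget is never executed.
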(event `self.ReceiveBeginPlay`
  (bind _returnvalue (`|CreateWidget` "/Game/FarmingDungeon/Blueprints/Widgets/WBP_InventaireCamionette.WBP_InventaireCamionette_C"))
  (set `self.WBP_InventaireCamionette` _returnvalue)
  (bind _asbp_game_instance (cast `/Game/FarmingDungeon/Blueprints/Manager/BP_GameInstance` (`GameplayStatics.GetGameInstance`)))
  (set `self.Ref_BP_GameInstance` _asbp_game_instance))

(fn `IsInteractible`
  (returns (Interactable :type Boolean))
  (return true))

(fn `OnInteract`
  (params (Player :type "/Game/FarmingDungeon/Blueprints/Characters/BP_Player Object Reference"))
  (bind _wbp_inventairecamionette (`self.WBP_InventaireCamionette`))
  (bind _ref_bp_gameinstance (`self.Ref_BP_GameInstance`))
  (bind _returnvalue (pcsubsystem `EnhancedInputLocalPlayerSubsystem` (`GameplayStatics.GetPlayerController` 0)))
  (bind _inventaire_player (`/Game/FarmingDungeon/Blueprints/Manager/BP_GameInstance.Inventaire_Player` _ref_bp_gameinstance))
  ;[1 1 1] BPI_Interface
  (message `EnhancedInputSubsystemInterface.AddMappingContext` _returnvalue "/Game/FarmingDungeon/Blueprints/Manager/Inputs/InputActions/IMC_Menu.IMC_Menu" 0 (struct))
  (message `EnhancedInputSubsystemInterface.RemoveMappingContext` _returnvalue "/Game/FarmingDungeon/Blueprints/Manager/Inputs/InputActions/IMC_Game.IMC_Game" (struct))
  (set `PlayerController.bShowMouseCursor` true (`GameplayStatics.GetPlayerController` 0))
  (for _index (range (`KismetArrayLibrary.Array_Length` _inventaire_player))
    (`/Game/FarmingDungeon/Blueprints/Widgets/WBP_InventaireCamionette.UpdateInventory` _wbp_inventairecamionette _index (`|GetArrayItem` (`/Game/FarmingDungeon/Blueprints/Manager/BP_GameInstance.NombreItem_Inventaire_Player` _ref_bp_gameinstance) _index) (`|GetArrayItem` _inventaire_player _index)))
  (`UserWidget.AddToViewport` _wbp_inventairecamionette 0)
  (return))

(fn `UserConstructionScript`)