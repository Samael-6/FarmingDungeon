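; BP_FlyingPickaxe is a flying pickaxe weapon that damages the actors it touches, excluding the player.
; While GoToLocation is set, Tick steps it toward LocationToGO at a fixed per-frame distance, without delta-time scaling, feeding only X and Y.
; Sphere overlaps apply damage through the target's BPC_PV component.
; Targets implementing BPI_AnimAttack also trigger a hit sound and that component's hit-animation message.
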(event `self.ReceiveTick`
  (params (DeltaSeconds :type "Float (single-precision)"))
  (bind _returnvalue (`self.K2_GetActorLocation`))
  (if (`self.GoToLocation?`)
    (`self.K2_SetActorLocation` (`KismetMathLibrary.MakeVector` (.x (+ _returnvalue (* (`KismetMathLibrary.Normal` (- (`self.Location To GO`) _returnvalue)) 2.0))) (.y (+ _returnvalue (* (`KismetMathLibrary.Normal` (- (`self.Location To GO`) _returnvalue)) 2.0)))))))

(event `self.ReceiveBeginPlay`
  (`self.SetVariables`))

(event `SetVariables`
  (bind _asbp_game_instance (cast `/Game/FarmingDungeon/Blueprints/Manager/BP_GameInstance` (`GameplayStatics.GetGameInstance`)))
  (set `self.Ref_BP_GameInstance` _asbp_game_instance)
  (bind _asbp_player (cast `/Game/FarmingDungeon/Blueprints/Characters/BP_Player` (`GameplayStatics.GetPlayerPawn` 0)))
  (set `self.Ref_BP_Player` _asbp_player))

(event `self.Sphere.OnComponentBeginOverlap`
  (params (OverlappedComponent :type "PrimitiveComponent Object Reference") (OtherActor :type "Actor Object Reference") (OtherComp :type "PrimitiveComponent Object Reference") (OtherBodyIndex :type Integer) (bFromSweep :type Boolean) (SweepResult :type "HitResult Structure (by ref)"))
  (bind _returnvalue (`self.GetComponentByClass` OtherActor "/Game/FarmingDungeon/Blueprints/Components/BPC_PV.BPC_PV_C"))
  (bind _ref_bp_player (`self.Ref_BP_Player`))
  (`/Engine/EditorBlueprintResources/StandardMacros.IsValid` _ref_bp_player
    (:`Is Valid`
      (if (not (== OtherActor _ref_bp_player))
        (`/Engine/EditorBlueprintResources/StandardMacros.IsValid` _returnvalue
          (:`Is Valid`
            (if (`KismetSystemLibrary.DoesImplementInterface` OtherActor "/Game/FarmingDungeon/Blueprints/Interfaces/BPI_AnimAttack.BPI_AnimAttack_C")
              (`GameplayStatics.PlaySound2D` "/Game/FarmingDungeon/Audio/SE/Axe_HIT.Axe_HIT" 1.0 1.0 0.0 null null)
              (message `/Game/FarmingDungeon/Blueprints/Interfaces/BPI_AnimAttack.AnimGetHit` _returnvalue))
            (`/Game/FarmingDungeon/Blueprints/Components/BPC_PV.Get_Hit` _returnvalue 1.0)))))))

(fn `UserConstructionScript`)