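; Axe weapon actor that sets its Attack value at BeginPlay and drives the player's axe moves.
; Basic and charged attacks play light or heavy montages, restore walk speed, and hold IsAttacking for the montage length, each gated by a DoOnce against retriggering.
; SlowWalk quarters the player's walk speed and plays a slow-walk montage, resetting its DoOnce immediately rather than waiting for the montage.
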(event `self.ReceiveBeginPlay`
  (set `self.Attack` 1.0))

(event `/Game/FarmingDungeon/Blueprints/Interfaces/BPI_Weapon.ChargedAttack`
  (params (BP_Player :type "/Game/FarmingDungeon/Blueprints/Characters/BP_Player Object Reference"))
  (`/Engine/EditorBlueprintResources/StandardMacros.DoOnce` false :!label _label
    (:`Completed`
      (set `/Game/FarmingDungeon/Blueprints/Characters/BP_Player.IsAttacking` true BP_Player)
      (bind _returnvalue (`Character.PlayAnimMontage` BP_Player "/Game/FarmingDungeon/Model3D/Personnages/felix/ANIM/Attacks/FELIX_HEAVY_AXE_Montage.FELIX_HEAVY_AXE_Montage" 1.0 "None"))
      (set `CharacterMovementComponent.MaxWalkSpeed` (`/Game/FarmingDungeon/Blueprints/Characters/BP_Player.SpeedWalk` BP_Player) (`Character.CharacterMovement` BP_Player))
      (`KismetSystemLibrary.Delay` _returnvalue)
      (set `/Game/FarmingDungeon/Blueprints/Characters/BP_Player.IsAttacking` false BP_Player)
      (goto _label :!via `Reset`))))

(event `/Game/FarmingDungeon/Blueprints/Interfaces/BPI_Weapon.BasicAttack`
  (params (BP_Player :type "/Game/FarmingDungeon/Blueprints/Characters/BP_Player Object Reference"))
  (`/Engine/EditorBlueprintResources/StandardMacros.DoOnce` false :!label _label_2
    (:`Completed`
      (set `/Game/FarmingDungeon/Blueprints/Characters/BP_Player.IsAttacking` true BP_Player)
      (bind _returnvalue (`Character.PlayAnimMontage` BP_Player "/Game/FarmingDungeon/Model3D/Personnages/felix/ANIM/Attacks/FELIX_LIGHT_AXE_Montage.FELIX_LIGHT_AXE_Montage" 1.0 "None"))
      (set `CharacterMovementComponent.MaxWalkSpeed` (`/Game/FarmingDungeon/Blueprints/Characters/BP_Player.SpeedWalk` BP_Player) (`Character.CharacterMovement` BP_Player))
      (`KismetSystemLibrary.Delay` _returnvalue)
      (set `/Game/FarmingDungeon/Blueprints/Characters/BP_Player.IsAttacking` false BP_Player)
      (goto _label_2 :!via `Reset`))))

(event `/Game/FarmingDungeon/Blueprints/Interfaces/BPI_Weapon.SlowWalk`
  (params (BP_Player :type "/Game/FarmingDungeon/Blueprints/Characters/BP_Player Object Reference"))
  (set `CharacterMovementComponent.MaxWalkSpeed` (/ (`/Game/FarmingDungeon/Blueprints/Characters/BP_Player.SpeedWalk` BP_Player) 4.0) (`Character.CharacterMovement` BP_Player))
  (`/Engine/EditorBlueprintResources/StandardMacros.DoOnce` false :!label _label_3
    (:`Completed`
      (`Character.PlayAnimMontage` BP_Player "/Game/FarmingDungeon/Model3D/Personnages/felix/ANIM/Attacks/FELIX_SLOW_WALK_Montage.FELIX_SLOW_WALK_Montage" 1.0 "None")
      (goto _label_3 :!via `Reset`))))

(fn `UserConstructionScript`
  (`parent.UserConstructionScript`))