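; Test actor that, judging by its name, serves to switch a villager's condition, and labels itself with the referenced villager's name.
; On player overlap, it disables its trigger box and spawns the configured number of ItemNeeded actors at its own transform.
; If the villager is BP_Mary, it also spawns extra BP_LootFraise pickups.
; The direct UpdateVillagerCondition call is disconnected, so the actor only supplies items.
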(event `self.ReceiveBeginPlay`
  (bind _asbp_game_instance (cast `/Game/FarmingDungeon/Blueprints/Manager/BP_GameInstance` (`GameplayStatics.GetGameInstance`)))
  (set `self.As BP Game Instance` _asbp_game_instance)
  (`KismetSystemLibrary.DelayUntilNextTick`)
  (bind _output_get (set `self.Text` (`KismetTextLibrary.Conv_StringToText` (`|GetEnumeratorNameAsString` (`/Game/FarmingDungeon/Blueprints/Characters/Villageois/BP_VillagerParent.E_VillagerName` (`self.VillagerRef`))))))
  (`TextRenderComponent.K2_SetText` (`self.TextRender`) _output_get))

(event `self.Box.OnComponentBeginOverlap`
  (params (OverlappedComponent :type "PrimitiveComponent Object Reference") (OtherActor :type "Actor Object Reference") (OtherComp :type "PrimitiveComponent Object Reference") (OtherBodyIndex :type Integer) (bFromSweep :type Boolean) (SweepResult :type "HitResult Structure (by ref)"))
  (cast `/Game/FarmingDungeon/Blueprints/Characters/BP_Player` OtherActor)
  (`PrimitiveComponent.SetCollisionEnabled` (`self.Box`) "NoCollision")
  (for _ (range (`self.NumberOfItems`))
    (`|SpawnActorFromClass` (`self.ItemNeeded`) (`self.GetTransform`) "Undefined" "MultiplyWithRoot" null null))
  (cast `/Game/FarmingDungeon/Blueprints/Characters/Villageois/BP_Mary` (`self.VillagerRef`))
  (for _ (range 5)
    (`|SpawnActorFromClass` "/Game/FarmingDungeon/Blueprints/Actors/BP_Ressources/RessourcesForest/BP_LootFraise.BP_LootFraise_C" (`self.GetTransform`) "Undefined" "MultiplyWithRoot" null null)))

(fn `UserConstructionScript`)