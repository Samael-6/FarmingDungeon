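; Level manager that builds a stage as a list of room level names drawn randomly from the F or M level list.
; CreateStageF and CreateStageM call MakeStage, which appends NumberOfRoom minus one entries to CurrentList, ending with "Lvl_Repos1", and prints debug output.
; Random picks aim to avoid consecutive repeats, but re-roll between check and add, and always use LevelListF's length as range.
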(event `self.ReceiveBeginPlay`)

(event `CreateStageF`
  (params (NumberOfRoom :type Integer))
  (`self.MakeStage` (`self.LevelListF`) NumberOfRoom))

(event `CreateStageM`
  (params (NumberOfRoom :type Integer))
  (`self.MakeStage` (`self.LevelListM`) NumberOfRoom))

(fn `MakeStage`
  (params (ListLevel :type "Array of Name") (NumberOfRoom :type Integer))
  (bind _output (`|GetArrayItem` ListLevel (`KismetMathLibrary.RandomIntegerInRange` 0 (- (`KismetArrayLibrary.Array_Length` (`self.LevelListF`)) 1))))
  (bind _output_get (set `self.NumberOfRoom` (- NumberOfRoom 1)))
  (while (> _output_get 0)
    (if (== 1 (`self.NumberOfRoom`))
      (bind _returnvalue (`KismetArrayLibrary.Array_Add` (`self.CurrentList`) "Lvl_Repos1"))
      (set `self.Index` _returnvalue)
      (bind _output_get_2 (set `self.NumberOfRoom` (- (`self.NumberOfRoom`) 1) :!label _label))
      (`KismetSystemLibrary.PrintString` (`KismetStringLibrary.Conv_IntToString` _output_get_2) true true (struct :`R` 0.78125 :`G` 0.276935 :`B` 0.011393 :`A` 1.0) 20.0)
      (`KismetSystemLibrary.PrintString` (`KismetStringLibrary.Conv_IntToString` (`self.Index`)) true true (struct :`G` 0.057873 :`B` 1.0 :`A` 1.0) 20.0)
      (elif (not (== (`|GetArrayItem` (`self.CurrentList`) (`self.Index`)) _output))
        (`KismetSystemLibrary.PrintString` (`KismetStringLibrary.Conv_NameToString` _output) true true (struct :`R` 0.040705 :`G` 1.0 :`A` 1.0) 45.0)
        (bind _returnvalue_2 (`KismetArrayLibrary.Array_Add` (`self.CurrentList`) _output))
        (set `self.Index` _returnvalue_2)
        (goto _label)))))

(fn `UserConstructionScript`)