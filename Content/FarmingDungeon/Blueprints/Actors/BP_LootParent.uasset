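; BP_LootParent is the loot actor base for the farming dungeon, with a plane that can be turned toward a camera.
; BeginPlay caches the player and game instance, and SetClassBPC copies the class name into the BPCLoot component and prints it.
; LookCamera rotates the root toward the dungeon camera, falling back to the player's follow camera, where the plane's forward vector serves as the start point.
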(event `self.ReceiveBeginPlay`
  (bind _asbp_player (cast `/Game/FarmingDungeon/Blueprints/Characters/BP_Player` (`GameplayStatics.GetPlayerPawn` 0)))
  (set `self.Ref_BP_Player` _asbp_player)
  (bind _asbp_game_instance (cast `/Game/FarmingDungeon/Blueprints/Manager/BP_GameInstance` (`GameplayStatics.GetGameInstance`)))
  (set `self.Ref_BP_GameInstance` _asbp_game_instance))

(event `SetClassBPC`
  ;[1 1 1] Mets la bonne class dans le BPC
  (bind _output_get (set `/Game/FarmingDungeon/Blueprints/Components/BPC_Loot.ClassName` (`self.ClassName`) (`self.BPC_Loot`)))
  (`KismetSystemLibrary.PrintString` (`|GetEnumeratorNameAsString` _output_get) true true (struct :`G` 0.057873 :`B` 1.0 :`A` 1.0)))

(event `LookCamera`
  ;[1 1 1] Permet de fixer la caméra du donjon
  (bind _returnvalue (`GameplayStatics.GetActorOfClass` "/Game/FarmingDungeon/Blueprints/Actors/BP_CameraDungeon.BP_CameraDungeon_C"))
  (`/Engine/EditorBlueprintResources/StandardMacros.IsValid` _returnvalue
    (:`Is Valid`
      (bind _output_get (set `self.Ref_BP_CameraDungeon` _returnvalue))
      (`self.MakeLookAt` (`SceneComponent.K2_GetComponentLocation` (`self.Plane`)) (`SceneComponent.K2_GetComponentLocation` (`Actor.RootComponent` _output_get))))
    (:`Is Not Valid`
      (set `self.Ref_BP_CameraPlayer` (`/Game/FarmingDungeon/Blueprints/Characters/BP_Player.FollowCamera` (`self.Ref_BP_Player`)))
      (`self.MakeLookAt` (`SceneComponent.GetForwardVector` (`self.Plane`)) (`SceneComponent.K2_GetComponentLocation` (`self.Ref_BP_CameraPlayer`))))))

(fn `MakeLookAt`
  (params (Start :type "Vector Structure") (End :type "Vector Structure"))
  (`SceneComponent.K2_SetWorldRotation` (`self.DefaultSceneRoot`) (`KismetMathLibrary.FindLookAtRotation` Start End) false false))

(fn `UserConstructionScript`)