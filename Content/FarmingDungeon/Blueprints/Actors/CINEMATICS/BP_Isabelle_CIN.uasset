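; BP_Isabelle_CIN is an always-interactable actor that triggers the ending cinematic.
; On interact it hides itself, the player and their weapon, disables input and removes the HUD.
; It reveals BP_ToShow actors, activates fireworks, plays the Cinematic_Montage sequence with music and effects, then adds the end credits widget after a delay.
; A delayed return to the main menu exists but is unconnected.
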(event `/Game/FarmingDungeon/Blueprints/Interfaces/BPI_Interact.OnInteract`
  (params (Player :type "/Game/FarmingDungeon/Blueprints/Characters/BP_Player Object Reference"))
  (`self.SetActorHiddenInGame` true)
  (bind _returnvalue (`GameplayStatics.GetActorOfClass` "/Game/FarmingDungeon/Blueprints/Characters/BP_Player.BP_Player_C"))
  (`self.DisableInput` _returnvalue (`GameplayStatics.GetPlayerController` 0))
  (`self.SetActorHiddenInGame` _returnvalue true)
  (`self.SetActorHiddenInGame` (`/Game/FarmingDungeon/Blueprints/Characters/BP_Player.Ref_ActualWeapon` _returnvalue) true)
  (`Widget.RemoveFromParent` (`/Game/FarmingDungeon/Blueprints/Characters/BP_Player.PlayerHUDRef` _returnvalue))
  (bind _outactors (`GameplayStatics.GetAllActorsOfClass` "/Game/FarmingDungeon/Blueprints/Actors/CINEMATICS/BP_ToShow.BP_ToShow_C"))
  (for _array_element _outactors
    (`self.SetActorHiddenInGame` _array_element false))
  (bind _outactors_2 (`GameplayStatics.GetAllActorsOfClass` "/Game/FarmingDungeon/Blueprints/Actors/CINEMATICS/BP_Fireworkd.BP_Fireworkd_C"))
  (for _array_element_2 _outactors_2
    (`ActorComponent.Activate` (`/Game/FarmingDungeon/Blueprints/Actors/CINEMATICS/BP_Fireworkd.NS_Firework_Complex` _array_element_2) true))
  (bind _outactor (`LevelSequencePlayer.CreateLevelSequencePlayer` "/Game/FarmingDungeon/Blueprints/Manager/Cinematic_Montage.Cinematic_Montage"))
  (`MovieSceneSequencePlayer.Play` (`LevelSequenceActor.SequencePlayer` _outactor))
  (bind _returnvalue_2 (`GameplayStatics.SpawnSound2D` "/Game/FarmingDungeon/Audio/Music/Painted_Dreams_Mock-Up.Painted_Dreams_Mock-Up" 1.0 1.0 0.0 null))
  (set `self.OST` _returnvalue_2)
  (`GameplayStatics.PlaySound2D` "/Game/FarmingDungeon/Audio/SE/Fireworks_Grand_Finale_Sound_Effect__FREE_TO_USE_.Fireworks_Grand_Finale_Sound_Effect__FREE_TO_USE_" 0.1 1.0 0.0 null null)
  (`KismetSystemLibrary.Delay` 13.0)
  (bind _returnvalue_3 (`|CreateWidget` "/Game/FarmingDungeon/Blueprints/Widgets/WBP_EndCredits.WBP_EndCredits_C"))
  (`UserWidget.AddToViewport` _returnvalue_3 0))

(fn `IsInteractible`
  (returns (Interactable :type Boolean))
  (return true))

(fn `UserConstructionScript`)