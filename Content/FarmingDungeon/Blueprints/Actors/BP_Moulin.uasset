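; Mill actor that converts items handed over by the player into products defined in TransformMap.
; Activating BPC_CanReceiveItem loads or stacks input, locks accepted items to that type, and starts a self-calling one-second Work loop that yields one product per ten ticks.
; BP_PaleMoulin, found by class lookup, moves until input runs out.
; Interacting passes one product to BPC_Loot, restoring the original accepted-item list once input and output are empty.
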(event `Work`
  (`KismetSystemLibrary.Delay` 1.0)
  (bind _output_get (set `self.CurrentWorkValue` (+ (`self.CurrentWorkValue`) 1)))
  (if (>= _output_get 10)
    (bind _finish_ (`self.CreateProduct`))
    (if _finish_
      (set `self.CurrentWorkValue` 0)
      (set `self.ItemContained` "NewEnumerator15")
      (bind _returnvalue (`GameplayStatics.GetActorOfClass` "/Game/Level_Design/Level_Blocking/_GENERATED/theoarene/BP_PaleMoulin.BP_PaleMoulin_C"))
      (`/Game/Level_Design/Level_Blocking/_GENERATED/theoarene/BP_PaleMoulin.StopMoving` _returnvalue)
      (else
        (set `self.CurrentWorkValue` 0)
        (`self.Work`)))
    (else
      (`self.Work`))))

(event `self.ReceiveBeginPlay`
  (set `self.CanReceiveArray` (`/Game/FarmingDungeon/Blueprints/Components/BPC_CanReceiveItem.CanReceiveItem` (`self.BPC_CanReceiveItem`))))

(event `self.BPC_CanReceiveItem.OnComponentActivated`
  (params (Component :type "ActorComponent Object Reference") (bReset :type Boolean))
  (if (`|EnumEquality` (`self.ItemContained`) "NewEnumerator15")
    (bind _output_get (set `self.ItemContained` (`/Game/FarmingDungeon/Blueprints/Components/BPC_CanReceiveItem.receivingItem` (`self.BPC_CanReceiveItem`))))
    (set `self.NumberOfItem` 1)
    (set `/Game/FarmingDungeon/Blueprints/Components/BPC_CanReceiveItem.CanReceiveItem` (`|MakeArray` _output_get) (`self.BPC_CanReceiveItem`))
    (set `self.IsEmpty?` false)
    (bind _returnvalue (`GameplayStatics.GetActorOfClass` "/Game/Level_Design/Level_Blocking/_GENERATED/theoarene/BP_PaleMoulin.BP_PaleMoulin_C"))
    (`/Game/Level_Design/Level_Blocking/_GENERATED/theoarene/BP_PaleMoulin.StartMoving` _returnvalue)
    (bind _returnvalue_2 (`GameplayStatics.GetActorOfClass` "/Game/FarmingDungeon/Blueprints/Characters/BP_Player.BP_Player_C"))
    (`/Game/FarmingDungeon/Blueprints/Characters/BP_Player.StopHoldAnimation` _returnvalue_2 true)
    (`self.Work`)
    (else
      (bind _output_get_2 (set `self.NumberOfItem` (+ (`self.NumberOfItem`) 1)))
      (bind _returnvalue_3 (`GameplayStatics.GetActorOfClass` "/Game/FarmingDungeon/Blueprints/Characters/BP_Player.BP_Player_C"))
      (`/Game/FarmingDungeon/Blueprints/Characters/BP_Player.StopHoldAnimation` _returnvalue_3 true))))

(event `/Game/FarmingDungeon/Blueprints/Interfaces/BPI_Interact.OnInteract`
  (params (Player :type "/Game/FarmingDungeon/Blueprints/Characters/BP_Player Object Reference"))
  (if (> (`self.NumberOfProductContained`) 0)
    (bind _output_get (set `/Game/FarmingDungeon/Blueprints/Components/BPC_Loot.ClassName` (`self.ProductContained`) (`self.BPC_Loot`)))
    (`/Game/FarmingDungeon/Blueprints/Components/BPC_Loot.CheckPositionInventory` (`self.BPC_Loot`) false)
    (bind _output_get_2 (set `self.NumberOfProductContained` (- (`self.NumberOfProductContained`) 1)))
    (if (<= _output_get_2 0)
      (set `self.ProductContained` "NewEnumerator15")
      (set `self.NumberOfProductContained` 0)
      (if (and (`|EnumEquality` (`self.ProductContained`) "NewEnumerator15") (`|EnumEquality` (`self.ItemContained`) "NewEnumerator15"))
        (set `/Game/FarmingDungeon/Blueprints/Components/BPC_CanReceiveItem.CanReceiveItem` (`self.CanReceiveArray`) (`self.BPC_CanReceiveItem`))
        (set `self.IsEmpty?` true)))))

(fn `CreateProduct`
  (returns (`Finish?` :type Boolean))
  (bind _transformmap (`self.TransformMap`))
  (bind _output_get (set `self.NumberOfItem` (- (`self.NumberOfItem`) 1)))
  (if (`|EnumEquality` (`self.ProductContained`) "NewEnumerator15")
    (bind _keys (`BlueprintMapLibrary.Map_Keys` _transformmap))
    (bind _values (`BlueprintMapLibrary.Map_Values` _transformmap))
    (set `self.ProductContained` (`|GetArrayItem` _values (`KismetArrayLibrary.Array_Find` _keys (`self.ItemContained`))))
    (set `self.NumberOfProductContained` 1)
    (else
      (set `self.NumberOfProductContained` (+ (`self.NumberOfProductContained`) 1))))
  (if (<= _output_get 0)
    (return true)
    (else
      (return false))))

(fn `IsInteractible`
  (returns (Interactable :type Boolean))
  (return true))

(fn `UserConstructionScript`)