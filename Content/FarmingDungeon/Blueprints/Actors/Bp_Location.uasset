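; Location volume actor that sets the player's current location name and shows it in the pause menu.
; When an actor with a BPC_Player component enters the Box, its BP_Player owner receives the Location value and the pause menu updates with level and location names.
; On BeginPlay, a short delay precedes the same update for a player already overlapping the Box.
; Leaving the Box does not clear the name.
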(event `self.ReceiveBeginPlay`
  (`KismetSystemLibrary.Delay` 0.1)
  (for _array_element (`PrimitiveComponent.GetOverlappingActors` (`self.Box`) "/Game/FarmingDungeon/Blueprints/Characters/BP_Player.BP_Player_C")
    (bind _returnvalue (`self.GetComponentByClass` _array_element "/Game/FarmingDungeon/Blueprints/Components/BPC_Player.BPC_Player_C"))
    (`/Engine/EditorBlueprintResources/StandardMacros.IsValid` _returnvalue
      (:`Is Valid`
        (bind _asbp_player (cast `/Game/FarmingDungeon/Blueprints/Characters/BP_Player` (`ActorComponent.GetOwner` _returnvalue)))
        (bind _output_get (set `/Game/FarmingDungeon/Blueprints/Characters/BP_Player.CurrentLocationName` (`self.Location`) _asbp_player))
        (`/Game/FarmingDungeon/Blueprints/Widgets/WBP_PauseMenu.UpdateLocation` (`/Game/FarmingDungeon/Blueprints/Characters/BP_Player.PauseMenu` _asbp_player) (`/Game/FarmingDungeon/Blueprints/Characters/BP_Player.CurrentLevelName` _asbp_player) _output_get)
        (break)))))

(event `self.Box.OnComponentBeginOverlap`
  (params (OverlappedComponent :type "PrimitiveComponent Object Reference") (OtherActor :type "Actor Object Reference") (OtherComp :type "PrimitiveComponent Object Reference") (OtherBodyIndex :type Integer) (bFromSweep :type Boolean) (SweepResult :type "HitResult Structure (by ref)"))
  (bind _returnvalue (`self.GetComponentByClass` OtherActor "/Game/FarmingDungeon/Blueprints/Components/BPC_Player.BPC_Player_C"))
  (`/Engine/EditorBlueprintResources/StandardMacros.IsValid` _returnvalue
    (:`Is Valid`
      (bind _asbp_player (cast `/Game/FarmingDungeon/Blueprints/Characters/BP_Player` (`ActorComponent.GetOwner` _returnvalue)))
      (bind _output_get (set `/Game/FarmingDungeon/Blueprints/Characters/BP_Player.CurrentLocationName` (`self.Location`) _asbp_player))
      (`/Game/FarmingDungeon/Blueprints/Widgets/WBP_PauseMenu.UpdateLocation` (`/Game/FarmingDungeon/Blueprints/Characters/BP_Player.PauseMenu` _asbp_player) (`/Game/FarmingDungeon/Blueprints/Characters/BP_Player.CurrentLevelName` _asbp_player) _output_get))))

(fn `UserConstructionScript`)