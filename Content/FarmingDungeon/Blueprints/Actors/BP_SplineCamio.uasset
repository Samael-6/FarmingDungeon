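; Spline-driven intro cutscene actor that drives BP_Camionette along a spline while its own camera follows on the Y axis, skipped when the tutorial is already finished.
; A timeline advances spline distance, with a brief pause and manual yaw turn near the end.
; At the spline's end, a white fade and car sounds hand the view back to the hidden player, then start BP_Isabelle and show the HUD.
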(event `self.ReceiveBeginPlay`)

(event `StratCinem`
  (bind _asbp_game_instance (cast `/Game/FarmingDungeon/Blueprints/Manager/BP_GameInstance` (`GameplayStatics.GetGameInstance`)))
  (if (`/Game/FarmingDungeon/Blueprints/Manager/BP_GameInstance.HasFinishedTuto` _asbp_game_instance)
    (bind _returnvalue (`GameplayStatics.GetActorOfClass` "/Game/FarmingDungeon/Blueprints/Characters/Villageois/BP_Isabelle.BP_Isabelle_C"))
    (`/Game/FarmingDungeon/Blueprints/Characters/Villageois/BP_Isabelle.Start` _returnvalue)
    (bind _asbp_player (cast `/Game/FarmingDungeon/Blueprints/Characters/BP_Player` (`GameplayStatics.GetPlayerPawn` 0)))
    (bind _output_get (set `self.BP_Player` _asbp_player))
    (`self.SetActorEnableCollision` _output_get true)
    (`self.SetActorHiddenInGame` _output_get false)
    (else
      (bind _returnvalue_2 (`GameplayStatics.GetActorOfClass` "/Game/FarmingDungeon/Blueprints/Actors/BP_Camionette.BP_Camionette_C"))
      (bind _output_get_2 (set `self.BP_Camionette` _returnvalue_2))
      (`self.K2_SetActorLocation` _output_get_2 (`.Position` (break `SplinePoint` (`SplineComponent.GetSplinePointAt` (`self.Spline`) 0 "Local"))) false false)
      (`PlayerController.SetViewTargetWithBlend` (`GameplayStatics.GetPlayerController` 0) self 0.0 "VTBlend_Linear" 0.0 false)
      (bind _asbp_player_2 (cast `/Game/FarmingDungeon/Blueprints/Characters/BP_Player` (`GameplayStatics.GetPlayerPawn` 0)))
      (bind _output_get_3 (set `self.BP_Player` _asbp_player_2))
      (`self.SetActorEnableCollision` _output_get_3 false)
      (`self.SetActorHiddenInGame` _output_get_3 true)
      (`self.AnimationCamio`))))

(event `AnimationCamio`
  (bind _bp_camionette (`self.BP_Camionette`))
  (bind _camera (`self.Camera`))
  (bind _bp_player (`self.BP_Player`))
  (bind (_returnvalue_roll _returnvalue_pitch _returnvalue_yaw) (`KismetMathLibrary.BreakRotator` (`self.K2_GetActorRotation` _bp_camionette)))
  (bind (_returnvalue_x _returnvalue_y) (`KismetMathLibrary.BreakVector` (`SplineComponent.GetLocationAtDistanceAlongSpline` (`self.Spline`) (`self.Distance`) "World")))
  (bind (_returnvalue_x_2 _returnvalue_y_2 _returnvalue_z) (`KismetMathLibrary.BreakVector` (`SceneComponent.K2_GetComponentLocation` _camera)))
  (bind (_direction _time) (`Timeline|Time` :!label _label)
    (:`Update`
      (`/Engine/EditorBlueprintResources/StandardMacros.IsValid` (`self.BP_Camionette`)
        (:`Is Valid`
          (set `self.Distance` (+ (* _time 5.0) (`self.Distance`)))
          (`self.K2_SetActorLocation` (`self.BP_Camionette`) (`SplineComponent.GetLocationAtDistanceAlongSpline` (`self.Spline`) (`self.Distance`) "World") false false)
          (`SceneComponent.K2_SetWorldLocation` _camera (`KismetMathLibrary.MakeVector` _returnvalue_x_2 _returnvalue_y _returnvalue_z) false false)
          (if (<= (`self.Distance`) (/ (`SplineComponent.GetSplineLength` (`self.Spline`)) 1.35))
            (`self.K2_SetActorRotation` (`self.BP_Camionette`) (`SplineComponent.GetRotationAtDistanceAlongSpline` (`self.Spline`) (`self.Distance`) "World") false)
            (else
              (`|ExecutionSequence`
                (:`then_0`
                  (`/Engine/EditorBlueprintResources/StandardMacros.DoOnce` false
                    (:`Completed`
                      (`|ExecutionSequence`
                        (:`then_0`
                          (goto _label :!via `Stop`))
                        (:`then_1`
                          (`KismetSystemLibrary.Delay` 0.5)
                          (goto _label))))))
                (:`then_1`
                  (if (>= (`self.Distance`) (`SplineComponent.GetSplineLength` (`self.Spline`)))
                    (`/Engine/EditorBlueprintResources/StandardMacros.DoOnce` false
                      (:`Completed`
                        (bind _returnvalue (`|CreateWidget` "/Game/FarmingDungeon/Blueprints/Widgets/WBP_Transitions.WBP_Transitions_C"))
                        (`UserWidget.AddToViewport` _returnvalue 0)
                        (bind _fadein_wihte (`/Game/FarmingDungeon/Blueprints/Widgets/WBP_Transitions.FadeIn_Wihte` _returnvalue))
                        (`UserWidget.PlayAnimation` _returnvalue _fadein_wihte 0.0 1 "Forward" 1.0 false)
                        (`KismetSystemLibrary.Delay` (`WidgetAnimation.GetEndTime` _fadein_wihte))
                        (`self.SetActorEnableCollision` _bp_player true)
                        (`self.SetActorHiddenInGame` _bp_player false)
                        (`/Game/FarmingDungeon/Blueprints/Components/BPC_Player.SetMenuInput` (`/Game/FarmingDungeon/Blueprints/Characters/BP_Player.BPC_Player` _bp_player))
                        (`GameplayStatics.PlaySound2D` "/Game/FarmingDungeon/Audio/SE/carDoorShut.carDoorShut" 1.0 1.0 0.0 null null)
                        (`KismetSystemLibrary.Delay` 1.0)
                        (`GameplayStatics.PlaySound2D` "/Game/FarmingDungeon/Audio/SE/WalkingOnDirt.WalkingOnDirt" 1.0 1.0 0.0 null null)
                        (`KismetSystemLibrary.Delay` 1.75)
                        (`PlayerController.SetViewTargetWithBlend` (`GameplayStatics.GetPlayerController` 0) (`self.BP_Player`) 0.0 "VTBlend_Linear" 0.0 false)
                        (bind _fadeout_wihte (`/Game/FarmingDungeon/Blueprints/Widgets/WBP_Transitions.FadeOut_Wihte` _returnvalue))
                        (`UserWidget.PlayAnimation` _returnvalue _fadeout_wihte 0.0 1 "Forward" 1.0 false)
                        (`KismetSystemLibrary.Delay` (`WidgetAnimation.GetEndTime` _fadeout_wihte))
                        (bind _returnvalue_2 (`GameplayStatics.GetActorOfClass` "/Game/FarmingDungeon/Blueprints/Characters/Villageois/BP_Isabelle.BP_Isabelle_C"))
                        (`/Game/FarmingDungeon/Blueprints/Characters/Villageois/BP_Isabelle.Start` _returnvalue_2)
                        (`Widget.RemoveFromParent` _returnvalue)
                        (`/Game/FarmingDungeon/Blueprints/Characters/BP_Player.DisplayHUD` (`self.BP_Player`) true)
                        (goto _label :!via `Stop`)))
                    (else
                      (set `self.Rotation` (`KismetMathLibrary.FClamp` (+ (`self.Rotation`) (* _time 1.0)) 0.0 0.475))
                      (`self.K2_SetActorRotation` _bp_camionette (`KismetMathLibrary.MakeRotator` _returnvalue_roll _returnvalue_pitch (+ _returnvalue_yaw (`self.Rotation`))) false))))))))))))

(fn `UserConstructionScript`)