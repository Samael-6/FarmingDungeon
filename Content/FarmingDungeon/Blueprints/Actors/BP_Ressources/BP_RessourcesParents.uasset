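; Parent Blueprint for harvestable resources that drop loot when destroyed.
; SetVariables assigns the hit points (PV) on the BPCPV component and the loot class to drop.
; A custom Start event, rather than BeginPlay, binds the component's death dispatcher (EDMort).
; On death it spawns the loot at its transform, calls LookCamera on it, unbinds the dispatcher and destroys itself.
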(event `self.ReceiveBeginPlay`)

(event `Start`
  (add `/Game/FarmingDungeon/Blueprints/Components/BPC_PV.ED_Mort` (`self.BPC_PV`) (delegate `OnDestroyRessource`)))

(event `OnDestroyRessource`
  (bind _returnvalue (`|SpawnActorFromClass` (`self.Loot`) (`self.GetTransform` self) "Undefined" "MultiplyWithRoot" null null))
  (`/Game/FarmingDungeon/Blueprints/Actors/BP_LootParent.LookCamera` _returnvalue)
  (clear `/Game/FarmingDungeon/Blueprints/Components/BPC_PV.ED_Mort` (`self.BPC_PV`))
  (`self.K2_DestroyActor`))

(fn `SetVariables`
  (params (PV :type "Float (double-precision)") (Loot :type "/Game/FarmingDungeon/Blueprints/Actors/BP_LootParent Class Reference"))
  (set `/Game/FarmingDungeon/Blueprints/Components/BPC_PV.PV` PV (`self.BPC_PV`))
  (set `self.Loot` Loot))

(fn `UserConstructionScript`)