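; Parent monster Blueprint that handles health, attacking the player and short random wandering.
; An interface-style set of getters and setters exposes monster HP and hittable state, and Tick destroys the actor once HP reaches zero.
; While IsAttacking is set, Attack subtracts the monster's attack value from the player HP stored in the GameInstance.
; RandomMove uses AIMoveTo toward a random nearby point around the mesh.
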(event `self.ReceiveBeginPlay`
  (bind _asbp_game_instance (cast `/Game/FarmingDungeon/Blueprints/Manager/BP_GameInstance` (`GameplayStatics.GetGameInstance`)))
  (set `self.Ref_BP_GameInstance` _asbp_game_instance)
  (bind _asbp_player (cast `/Game/FarmingDungeon/Blueprints/Characters/BP_Player` (`GameplayStatics.GetPlayerPawn` 0)))
  (set `self.Ref_BP_Player` _asbp_player))

(event `self.ReceiveTick`
  (params (DeltaSeconds :type "Float (single-precision)"))
  (if (<= (`self.PV_Monstre`) 0.0)
    (`self.K2_DestroyActor`)))

(event `Attack`
  ;[1 1 1] Gestion PVet Damage avec BPI
  (if (`self.IsAttacking`)
    (bind _pv_remaining (`/Game/FarmingDungeon/Blueprints/Interfaces/BPI_Attack.DoAttack` (`/Game/FarmingDungeon/Blueprints/Manager/BP_GameInstance.PV_Player` (`self.Ref_BP_GameInstance`)) (`self.Attack_Monstre`)))
    (set `/Game/FarmingDungeon/Blueprints/Manager/BP_GameInstance.PV_Player` _pv_remaining (`self.Ref_BP_GameInstance`))))

(event `/Game/FarmingDungeon/Blueprints/Interfaces/BPI_Attack.SetState`
  (params (State :type Boolean))
  ;[1 1 1] Gestion PVet Damage avec BPI
  (set `self.IsHittable` State))

(event `/Game/FarmingDungeon/Blueprints/Interfaces/BPI_Attack.Set_PV`
  (params (PV :type "Float (double-precision)"))
  ;[1 1 1] Gestion PVet Damage avec BPI
  (bind _output_get (set `self.PV_Monstre` PV))
  (`KismetSystemLibrary.PrintString` (`KismetStringLibrary.Conv_DoubleToString` _output_get)))

(event `RandomMove`
  (bind (_returnvalue_x _returnvalue_y _returnvalue_z) (`KismetMathLibrary.BreakVector` (`SceneComponent.K2_GetComponentLocation` (`self.Mesh`))))
  ;[1 1 1] Déplacement random des monstres
  (`|AIMoveTo` self (`KismetMathLibrary.MakeVector` (`KismetMathLibrary.RandomFloatInRange` (- _returnvalue_x 50.0) (+ _returnvalue_x 50.0)) (`KismetMathLibrary.RandomFloatInRange` (- _returnvalue_y 50.0) (+ _returnvalue_y 50.0)) _returnvalue_z) null))

(fn `DoAttack`
  (params (PV :type "Float (double-precision)") (Attack :type "Float (double-precision)"))
  (returns (PV_Remaining :type "Float (double-precision)"))
  (return (- PV Attack)))

(fn `Get_PV`
  (returns (PV :type "Float (double-precision)"))
  (return (`self.PV_Monstre`)))

(fn `GetState`
  (returns (StateMonstre :type Boolean))
  (return (`self.IsHittable`)))

(fn `UserConstructionScript`)