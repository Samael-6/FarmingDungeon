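; Monster spawner actor for dungeon levels that spawns its chosen monster class at its own transform when SpawnMonster runs while active.
; The construction script picks the monster list and dungeon level matching the game instance's level flag, though that reference is only set in BeginPlay.
; MonsterChoice derives level-scaled odds and rolls for the first two entries, then overwrites the choice with the loop's last element.
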(event `self.ReceiveBeginPlay`
  (bind _asbp_game_instance (cast `/Game/FarmingDungeon/Blueprints/Manager/BP_GameInstance` (`GameplayStatics.GetGameInstance`)))
  (set `self.BP_GameInstance_Ref` _asbp_game_instance)
  (set `self.BP_GameMode_Ref` (`GameplayStatics.GetGameMode`)))

(fn `GetMonsterFromList`
  (params (ListeMonster :type "Array of /Game/FarmingDungeon/Blueprints/Actors/BP_MonstreParent Class Reference") (Index :type Integer))
  (returns (Monstre :type "/Game/FarmingDungeon/Blueprints/Actors/BP_MonstreParent Class Reference"))
  (return (`|GetArrayItem` ListeMonster Index)))

(fn `MonsterChoice`
  (params (ListeMonstre :type "Array of /Game/FarmingDungeon/Blueprints/Actors/BP_MonstreParent Class Reference") (LvlDungeuon :type Integer))
  (set `self.TauxMonstresMoy` (- (* LvlDungeuon 10) 10))
  (set `self.TauxMonstresPetits` (- (`self.TauxMonstresPetits`) (/ (`self.TauxMonstresMoy`) 2)))
  (for (_array_element _array_index) ListeMonstre
    (switch `int` _array_index
      (:`0`
        (if (> (`self.TauxMonstresMoy`) (`KismetMathLibrary.RandomIntegerInRange` 0 100))
          (set `self.Monstre` _array_element)))
      (:`1`
        (if (> (`self.TauxMonstresPetits`) (`KismetMathLibrary.RandomIntegerInRange` 0 100))
          (set `self.Monstre` _array_element)))))
  (set `self.Monstre` _array_element))

(fn `SpawnMonster`
  (if (`self.IsActive`)
    (`|SpawnActorFromClass` (`self.Monstre`) (`self.GetTransform` self) "Undefined" "MultiplyWithRoot" null null)))

(fn `UserConstructionScript`
  (bind _bp_gameinstance_ref (`self.BP_GameInstance_Ref`))
  (bind _bp_gameinstance_ref_2 (`self.BP_GameInstance_Ref`))
  (if (`|GetArrayItem` (`/Game/FarmingDungeon/Blueprints/Manager/BP_GameInstance.IsLevel` (`self.BP_GameInstance_Ref`)) 1)
    (`self.MonsterChoice` (`/Game/FarmingDungeon/Blueprints/Manager/BP_GameInstance.ListeMonstresF` _bp_gameinstance_ref_2) (`/Game/FarmingDungeon/Blueprints/Manager/BP_GameInstance.Lvl_DungeounF` _bp_gameinstance_ref_2))
    (elif (`|GetArrayItem` (`/Game/FarmingDungeon/Blueprints/Manager/BP_GameInstance.IsLevel` _bp_gameinstance_ref) 2)
      (`self.MonsterChoice` (`/Game/FarmingDungeon/Blueprints/Manager/BP_GameInstance.ListeMonstresM` _bp_gameinstance_ref) (`/Game/FarmingDungeon/Blueprints/Manager/BP_GameInstance.Lvl_DungeunM` _bp_gameinstance_ref)))))